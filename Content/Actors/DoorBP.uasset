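; Door actor that swings open and closed, with a randomized wobble material.
; An overlap box sets or clears it as the Roodie first-person character's CurrentDoor; OpenCloseDoor toggles a yaw timeline, locked by DoOnce until one second after it finishes.
; Construction shares one dynamic material between door and frame and applies the initial open rotation.
; BeginPlay randomizes wobble speed and modes, with WobbleMode4 overwritten by each roll so only the last sticks.
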(event OnComponentBeginOverlap(Box)
  (params (OverlappedComponent :type Primitive%20Component%20Object%20Reference) (OtherActor :type Actor%20Object%20Reference) (OtherComp :type Primitive%20Component%20Object%20Reference) (OtherBodyIndex :type Integer) (bFromSweep :type Boolean) (SweepResult :type Hit%20Result%20Structure%20%28by%20ref%29))
  (bind _asroodie_first_person_bp (Utilities|Casting|CastToRoodie_FirstPerson_BP OtherActor))
  (Variables|/Game/Roodie_BP/Blueprints/Roodie_FirstPerson_BP.Roodie_FirstPerson_BP_C|SetCurrentDoor _asroodie_first_person_bp self))

(event OnComponentEndOverlap(Box)
  (params (OverlappedComponent :type Primitive%20Component%20Object%20Reference) (OtherActor :type Actor%20Object%20Reference) (OtherComp :type Primitive%20Component%20Object%20Reference) (OtherBodyIndex :type Integer))
  (bind _asroodie_first_person_bp (Utilities|Casting|CastToRoodie_FirstPerson_BP OtherActor))
  (Variables|/Game/Roodie_BP/Blueprints/Roodie_FirstPerson_BP.Roodie_FirstPerson_BP_C|SetCurrentDoor _asroodie_first_person_bp 0))

(event Custom|OpenCloseDoor
  (Utilities|FlowControl|DoOnce false :!label _label
    (:Completed
      (if (Variables|Default|GetIsClosed)
        (Variables|Default|SetIsClosed false)
        (bind _track_opendoor (Timeline|Timeline_OpenDoor PlayFromStart)
          (:Update
            (Transformation|SetRelativeRotation (Variables|Default|GetDoor) (Math|Rotator|MakeRotator 0.0 0.0 (* _track_opendoor (Variables|Default|GetDoorPosition))) false false))
          (:Finished
            (Utilities|FlowControl|Delay 1.0)
            (goto _label Reset)))
        (else
          (Variables|Default|SetIsClosed true)
          (Timeline|Timeline_OpenDoor Reverse))))))

(event EventTick
  (params (DeltaSeconds :type Float%20%28single-precision%29)))

(event EventBeginPlay
  (bind _material (Variables|Default|GetMaterial))
  (bind _wobble (Variables|Default|GetWobble))
  (Rendering|Material|SetScalarParameterValue _material "Wobble Speed" (+ (* (Math|Random|RandomIntegerinRange 0 3) _wobble) _wobble) :!class /Script/Engine.MaterialInstanceDynamic)
  (Utilities|FlowControl|Sequence
    (:then_0
      (bind (_switchwobble _wobbleeffect) (CallFunction|GetRandomFloat))
      (Rendering|Material|SetScalarParameterValue _material "WobbleMode1" _switchwobble :!class /Script/Engine.MaterialInstanceDynamic)
      (Rendering|Material|SetScalarParameterValue _material "WobbleMode4" _wobbleeffect :!class /Script/Engine.MaterialInstanceDynamic))
    (:then_1
      (bind (_switchwobble_2 _wobbleeffect_2) (CallFunction|GetRandomFloat))
      (Rendering|Material|SetScalarParameterValue _material "WobbleMode2" _switchwobble_2 :!class /Script/Engine.MaterialInstanceDynamic)
      (Rendering|Material|SetScalarParameterValue _material "WobbleMode4" _wobbleeffect_2 :!class /Script/Engine.MaterialInstanceDynamic))
    (:then_2
      (bind (_switchwobble_3 _wobbleeffect_3) (CallFunction|GetRandomFloat))
      (Rendering|Material|SetScalarParameterValue _material "WobbleMode3" _switchwobble_3 :!class /Script/Engine.MaterialInstanceDynamic)
      (Rendering|Material|SetScalarParameterValue _material "WobbleMode4" _wobbleeffect_3 :!class /Script/Engine.MaterialInstanceDynamic))))

(fn ConstructionScript
  (bind _doorframe (Variables|Default|GetDoorFrame))
  (bind _returnvalue (Rendering|Material|CreateDynamicMaterialInstance _doorframe 0 (Rendering|Material|GetMaterial _doorframe 0) "None" :!class /Script/Engine.PrimitiveComponent))
  (bind _output_get (Variables|Default|SetMaterial _returnvalue))
  (Rendering|Material|SetMaterial _doorframe 0 _output_get)
  (bind _returnvalue_2 (Rendering|Material|GetScalarParameterValue _output_get "Wobble Speed" :!class /Script/Engine.MaterialInstanceDynamic))
  (Variables|Default|SetWobble _returnvalue_2)
  (if (not (Variables|Default|GetIsClosed))
    (Transformation|SetRelativeRotation (Variables|Default|GetDoor) (Math|Rotator|MakeRotator 0.0 0.0 (Variables|Default|GetDoorPosition)) false false)))

(fn GetRandomFloat
  (bind _returnvalue (Math|Random|RandomFloatinRange 0.0001 2.0))
  (switch int (Math|Random|RandomIntegerinRange 0 1)
    (:0
      (return 0.0 _returnvalue))
    (:1
      (return 1.0 _returnvalue))))