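; AI controller for a decorative rat that wanders around and moves away from the player.
; A RandomWalk loop started on BeginPlay moves it to random reachable nearby points, pausing a random few seconds after each success or failure.
; Every Tick, it issues a short move directly away from the player when the summed signed XYZ offset, rather than true distance, is below a threshold.
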(event EventTick
  (params (DeltaSeconds :type Float%20%28single-precision%29))
  (bind _returnvalue (Pawn|GetControlledPawn))
  (bind _returnvalue_2 (Pawn|GetControlledPawn))
  (bind _returnvalue_3 (Game|GetPlayerCharacter 0))
  (bind _returnvalue_4 (Transformation|GetActorLocation _returnvalue))
  (bind _returnvalue_5 (Transformation|GetActorLocation _returnvalue_3))
  (bind _returnvalue_6 (Transformation|GetActorLocation _returnvalue_2))
  (bind _returnvalue_7 (- _returnvalue_6 _returnvalue_5))
  (bind (_x _y _z) (Math|Vector|BreakVector _returnvalue_7))
  (if (< (+ _x _y _z) 2e+02)
    (AI|AIMoveTo _returnvalue (+ _returnvalue_4 (* (Math|Vector|Normalize (- _returnvalue_4 (Transformation|GetActorLocation (Game|GetPlayerCharacter 0)))) 2e+01)) 0 0.0 false)))

(fn ConstructionScript)

(event Custom|Random%20Walk
  (bind _returnvalue (Pawn|GetControlledPawn))
  (AI|AIMoveTo _returnvalue (.RandomLocation (AI|Navigation|GetRandomReachablePointinRadius (Transformation|GetActorLocation _returnvalue) 3e+02 0 0)) 0 5.0 false :!label _label
    (:OnSuccess
      _)
    (:OnFail
      _))
  (Utilities|FlowControl|Delay (Math|Random|RandomFloatinRange 2.0 4.0))
  (goto _label))

(event EventBeginPlay
  (CallFunction|RandomWalk))