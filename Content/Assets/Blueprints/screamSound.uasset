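; screamSound is a one-shot trigger actor that plays a positioned sound when the Female_BP actor overlaps its box.
; It plays the configured sound at an offset from its root with attenuation, guarded by DoOnce and an AlreadyDone check.
; After the sound's duration plus a short delay, it saves the event under its object name and destroys itself.
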(event OnComponentBeginOverlap(Box)
  (params (OverlappedComponent :type Primitive%20Component%20Object%20Reference) (OtherActor :type Actor%20Object%20Reference) (OtherComp :type Primitive%20Component%20Object%20Reference) (OtherBodyIndex :type Integer) (bFromSweep :type Boolean) (SweepResult :type Hit%20Result%20Structure%20%28by%20ref%29))
  (bind _sound (Variables|Default|Getsound))
  (Utilities|Casting|CastToFemale_BP OtherActor)
  (bind _done (CallFunction|AlreadyDone))
  (if (not _done)
    (Utilities|FlowControl|DoOnce false
      (:Completed
        (Audio|PlaySoundatLocation _sound (+ (Transformation|GetWorldLocation (Variables|Default|GetDefaultSceneRoot)) (Variables|Default|GetLocation)) "0, 0, 0" 1.0 1.0 0.0 (Variables|Default|GetAttenuation%20Settings) 0 0)
        (Utilities|FlowControl|Delay (+ (Variables|/Script/Engine.SoundBase|GetDuration _sound) 3.0))
        (CallFunction|SaveEvent (Utilities|GetObjectName self))
        (Actor|DestroyActor)))))

(fn ConstructionScript)