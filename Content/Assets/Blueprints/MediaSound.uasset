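; MediaSound is a trigger-box actor that plays a sequence of three positional sounds when the first-person player Blueprint overlaps it.
; Each attenuated sound plays at the actor's root, with delays based on each clip's duration chaining them back to back.
; A DoOnce blocks retriggering until the sequence ends plus a short cooldown, then resets.
; A constant-true branch leaves the DestroyActor path unreachable.
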(event OnComponentBeginOverlap(Box)
  (params (OverlappedComponent :type Primitive%20Component%20Object%20Reference) (OtherActor :type Actor%20Object%20Reference) (OtherComp :type Primitive%20Component%20Object%20Reference) (OtherBodyIndex :type Integer) (bFromSweep :type Boolean) (SweepResult :type Hit%20Result%20Structure%20%28by%20ref%29))
  (bind _sound2 (Variables|Default|GetSound2))
  (bind _sound3 (Variables|Default|GetSound3))
  (bind _sound1 (Variables|Default|GetSound1))
  (Utilities|Casting|CastToRoodie_FirstPerson_BP OtherActor)
  (if true
    (Utilities|FlowControl|DoOnce false :!label _label
      (:Completed
        (Audio|PlaySoundatLocation _sound1 (Transformation|GetWorldLocation (Variables|Default|GetDefaultSceneRoot)) "0, 0, 0" 1.0 1.0 0.0 (Variables|Default|GetAttenuation%20Settings) 0 0)
        (Utilities|FlowControl|Delay (Variables|/Script/Engine.SoundBase|GetDuration _sound1))
        (Audio|PlaySoundatLocation _sound2 (Transformation|GetWorldLocation (Variables|Default|GetDefaultSceneRoot)) "0, 0, 0" 1.0 1.0 0.0 (Variables|Default|GetAttenuation%20Settings) 0 0)
        (Utilities|FlowControl|Delay (Variables|/Script/Engine.SoundBase|GetDuration _sound2))
        (Audio|PlaySoundatLocation _sound3 (Transformation|GetWorldLocation (Variables|Default|GetDefaultSceneRoot)) "0, 0, 0" 1.0 1.0 0.0 (Variables|Default|GetAttenuation%20Settings) 0 0)
        (Utilities|FlowControl|Delay (+ (Variables|/Script/Engine.SoundBase|GetDuration _sound3) 5.0))
        (goto _label Reset)))
    (else
      (Actor|DestroyActor))))

(event EventBeginPlay)

(event Collision|EventActorBeginOverlap
  (params (OtherActor :type Actor%20Object%20Reference)))

(event EventTick
  (params (DeltaSeconds :type Float%20%28single-precision%29)))

(fn ConstructionScript)