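; Secret door actor that the first-person player opens with Interact while overlapping it, provided it is unlocked.
; Overlap toggles input and a gate, and the player's admin-mode event clears the lock.
; Opening plays a sound, then chains two timelines: a sideways slide along relative Y, followed by a yaw swing scaled by DoorPosition.
; It opens only once, as the DoOnce reset is unconnected and no closing logic exists.
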(event Custom|OpenAllDoors
  (Variables|Default|SetLocked false))

(event EventBeginPlay
  (bind _defaultsceneroot (Variables|Default|GetDefaultSceneRoot))
  (bind _relativelocation (Variables|/Script/Engine.SceneComponent|GetRelativeLocation _defaultsceneroot))
  (Variables|Default|SetGameinstanceReference (.AsGame%20Instance%20Horror (Utilities|Casting|CastToGameInstanceHorror (Game|GetGameInstance))))
  (EventDispatchers|BindEventtoAdminMode (.AsRoodie%20First%20Person%20BP (Utilities|Casting|CastToRoodie_FirstPerson_BP (Game|Player|GetPlayerPawn 0))) (delegate Custom|OpenAllDoors))
  (Variables|Default|SetdefaultX (.x _relativelocation))
  (bind _output_get (Variables|Default|SetdefaultY (.y _relativelocation)))
  (Variables|Default|SetdefaultZ (.z _relativelocation))
  (Variables|Default|SetnewY (+ 6e+01 _output_get)))

(event EventTick
  (params (DeltaSeconds :type Float%20%28single-precision%29)))

(event Collision|EventActorBeginOverlap
  (params (OtherActor :type Actor%20Object%20Reference))
  (Utilities|Casting|CastToRoodie_FirstPerson_BP OtherActor)
  (Input|EnableInput (Game|GetPlayerController 0))
  (Variables|Default|SetIsLookingAt true)
  (Development|PrintString "BeginOverlap")
  (Utilities|FlowControl|Gate true) ; enters at Open
)

(event Collision|EventActorEndOverlap
  (params (OtherActor :type Actor%20Object%20Reference))
  (Utilities|Casting|CastToRoodie_FirstPerson_BP OtherActor)
  (Input|DisableInput (Game|GetPlayerController 0))
  (Variables|Default|SetIsLookingAt false)
  (Development|PrintString "EndOverlap")
  (Utilities|FlowControl|Gate true) ; enters at Close
)

(event Input|ActionEvents|InputActionInteract
  (params (Key :type Key%20Structure :default "None"))
  (:Pressed
    (Utilities|FlowControl|Delay 0.2)
    (if (Variables|Default|GetIsLookingAt)
      (Utilities|FlowControl|Gate true
        (:Exit
          (if (not (Variables|Default|GetLocked))
            (Utilities|FlowControl|DoOnce false
              (:Completed
                (if (Variables|Default|GetIsClosed)
                  (Variables|Default|SetIsClosed false)
                  (Audio|PlaySoundatLocation "/Game/Sound/Tür/Türöffnen01_Cue.Türöffnen01_Cue" (Transformation|GetWorldLocation (Variables|Default|GetDefaultSceneRoot)) "0, 0, 0" 1.0 1.0 0.0 0 0 0)
                  (Development|PrintString "öffnet")
                  (bind _track_opendoor (Timeline|Timeline_2 PlayFromStart)
                    (:Update
                      (Transformation|SetRelativeLocation (Variables|Default|GetDefaultSceneRoot) (Math|Vector|MakeVector (Variables|Default|GetdefaultX) (Math|Float|Lerp (Variables|Default|GetdefaultY) (Variables|Default|GetnewY) _track_opendoor) (Variables|Default|GetdefaultZ)) false false))
                    (:Finished
                      (bind _track_opendoor_2 (Timeline|Timeline_0 PlayFromStart)
                        (:Update
                          (Transformation|SetRelativeRotation (Variables|Default|GetDefaultSceneRoot) (Math|Rotator|MakeRotator 0.0 0.0 (* _track_opendoor_2 (Variables|Default|GetDoorPosition))) false false))))))))))))))

(fn ConstructionScript)