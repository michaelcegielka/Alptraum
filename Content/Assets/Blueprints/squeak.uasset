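; Trigger volume that plays a random squeak sound when the first-person Roodie player enters its box.
; On overlap it casts the actor to Roodie_FirstPerson_BP and picks a random entry from the Sound array.
; The sound plays high above the player's mesh with a small random horizontal offset, so it comes from overhead.
; It has no cooldown or one-shot guard.
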(event OnComponentBeginOverlap(Box)
  (params (OverlappedComponent :type Primitive%20Component%20Object%20Reference) (OtherActor :type Actor%20Object%20Reference) (OtherComp :type Primitive%20Component%20Object%20Reference) (OtherBodyIndex :type Integer) (bFromSweep :type Boolean) (SweepResult :type Hit%20Result%20Structure%20%28by%20ref%29))
  (bind _sound (Variables|Default|Getsound))
  (bind _asroodie_first_person_bp (Utilities|Casting|CastToRoodie_FirstPerson_BP OtherActor))
  (Audio|PlaySoundatLocation (Utilities|Array|Get(acopy) _sound (Math|Random|RandomInteger (Utilities|Array|Length _sound))) (Math|Vector|MakeVector (+ (.x (Transformation|GetWorldLocation (Variables|/Script/Engine.Character|GetMesh _asroodie_first_person_bp))) (Math|Random|RandomFloatinRange 0.0 5e+01)) (+ (.y (Transformation|GetWorldLocation (Variables|/Script/Engine.Character|GetMesh _asroodie_first_person_bp))) (Math|Random|RandomFloatinRange 0.0 5e+01)) (+ (.z (Transformation|GetWorldLocation (Variables|/Script/Engine.Character|GetMesh _asroodie_first_person_bp))) 5e+02)) "0, 0, 0" 1.0 1.0 0.0 0 0 0))

(event EventBeginPlay)

(event Collision|EventActorBeginOverlap
  (params (OtherActor :type Actor%20Object%20Reference)))

(event EventTick
  (params (DeltaSeconds :type Float%20%28single-precision%29)))

(fn ConstructionScript)