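; Trigger actor that plays a random positional sound when the first-person Roodie player enters its box.
; It silences and blocks the level's first SoundSystem during playback, then resumes it after a clip duration plus padding.
; The delay rolls its own random index, so it may not match the played clip.
; DoOnce and DestroyActor are disconnected, leaving the trigger repeatable.
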(event OnComponentBeginOverlap(Box)
  (params (OverlappedComponent :type Primitive%20Component%20Object%20Reference) (OtherActor :type Actor%20Object%20Reference) (OtherComp :type Primitive%20Component%20Object%20Reference) (OtherBodyIndex :type Integer) (bFromSweep :type Boolean) (SweepResult :type Hit%20Result%20Structure%20%28by%20ref%29))
  (bind _sound (Variables|Default|Getsound))
  (bind _returnvalue (Utilities|Array|Length _sound))
  (bind _returnvalue_2 (Math|Random|RandomInteger _returnvalue))
  (bind _output (Utilities|Array|Get(acopy) _sound _returnvalue_2))
  (Utilities|Casting|CastToRoodie_FirstPerson_BP OtherActor)
  (bind _outactors (Actor|GetAllActorsOfClass "/Game/Sound/SoundSystem.SoundSystem_C"))
  (Variables|/Game/Sound/SoundSystem.SoundSystem_C|SetBlocked (Utilities|Array|Get(acopy) _outactors) true)
  (Default|StopSound (Utilities|Array|Get(acopy) _outactors))
  (Audio|PlaySoundatLocation _output (Transformation|GetWorldLocation (Variables|Default|GetDefaultSceneRoot)) "0, 0, 0" 1.0 1.0 0.0 (Variables|Default|GetAttenuation%20Settings) 0 0)
  (Utilities|FlowControl|Delay (+ (Variables|/Script/Engine.SoundBase|GetDuration _output) 3.0))
  (Default|PlaySound (Utilities|Array|Get(acopy) _outactors))
  (Variables|/Game/Sound/SoundSystem.SoundSystem_C|SetBlocked (Utilities|Array|Get(acopy) _outactors) false))

(event EventBeginPlay)

(event Collision|EventActorBeginOverlap
  (params (OtherActor :type Actor%20Object%20Reference)))

(event EventTick
  (params (DeltaSeconds :type Float%20%28single-precision%29)))

(fn ConstructionScript)