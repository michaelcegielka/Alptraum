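; Master commode Blueprint: furniture with a sliding drawer (Schublade) that can hold a collectable item.
; Box overlap with the first-person player enables input and opens the gate for Open/Close, which lerps drawer Y through timelines with sound and a DoOnce lock.
; On an open drawer, a live item is collected through InteractInterface before closing is possible.
; BeginPlay randomizes item yaw; SetGameItem configures a child-actor GameItem's type and scale.
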(event OnComponentBeginOverlap(Box)
  (params (OverlappedComponent :type Primitive%20Component%20Object%20Reference) (OtherActor :type Actor%20Object%20Reference) (OtherComp :type Primitive%20Component%20Object%20Reference) (OtherBodyIndex :type Integer) (bFromSweep :type Boolean) (SweepResult :type Hit%20Result%20Structure%20%28by%20ref%29))
  (bind _collectable (Variables|Default|Getcollectable))
  (bind _childactor (Variables|/Script/Engine.ChildActorComponent|GetChildActor _collectable))
  (Utilities|Casting|CastToRoodie_FirstPerson_BP OtherActor)
  (Input|EnableInput (Game|GetPlayerController 0))
  (Variables|Default|SetIsLookingAtComm true)
  (Utilities|FlowControl|Gate true) ; enters at Open
)

(event OnComponentEndOverlap(Box)
  (params (OverlappedComponent :type Primitive%20Component%20Object%20Reference) (OtherActor :type Actor%20Object%20Reference) (OtherComp :type Primitive%20Component%20Object%20Reference) (OtherBodyIndex :type Integer))
  (bind _collectable (Variables|Default|Getcollectable))
  (bind _childactor (Variables|/Script/Engine.ChildActorComponent|GetChildActor _collectable))
  (Utilities|Casting|CastToRoodie_FirstPerson_BP OtherActor)
  (Input|DisableInput (Game|GetPlayerController 0))
  (Variables|Default|SetIsLookingAtComm false)
  (Utilities|FlowControl|Gate true) ; enters at Close
)

(event Custom|Open/Close
  (params (OpenLocation :type Float%20%28single-precision%29) (Schublade :type Static%20Mesh%20Component%20Object%20Reference))
  (bind _collectable (Variables|Default|Getcollectable))
  (bind _childactor (Variables|/Script/Engine.ChildActorComponent|GetChildActor _collectable))
  (Variables|Default|SetOpen%20Location OpenLocation)
  (Variables|Default|SetSchublade Schublade)
  (Utilities|FlowControl|Delay 0.2)
  (if (Variables|Default|GetIsLookingAtComm)
    (Utilities|FlowControl|Gate true
      (:Exit
        (Utilities|FlowControl|DoOnce false :!label _label
          (:Completed
            (if (Variables|Default|GetIs%20Wardrobe%20Closed)
              (Audio|PlaySoundatLocation "/Game/Sound/Schublade/OpeningDrawer01_Cue.OpeningDrawer01_Cue" (Transformation|GetWorldLocation (Variables|Default|GetSchublade)) "0, 0, 0" 1.0 1.0 0.0 0 0 0)
              ;[1 1 1] Open Schublade
              (bind _open_close (Timeline|Timeline_0 PlayFromStart)
                (:Update
                  (Transformation|SetRelativeLocation (Variables|Default|GetSchublade) (Math|Vector|MakeVector (Variables|Default|GetDefault%20X) (Math|Float|Lerp (Variables|Default|GetClose%20Location) (Variables|Default|GetOpen%20Location) _open_close) (Variables|Default|GetDefault%20Z)) false false)
                  (Utilities|FlowControl|Delay 2.0 :!label _label_2)
                  (goto _label Reset))
                (:Finished
                  (Variables|Default|SetIs%20Wardrobe%20Closed false)))
              (elif (Variables|Default|GetItemAlive)
                (if (Utilities|DoesObjectImplementInterface _childactor "/Game/Game/InteractInterFace.InteractInterface_C")
                  (Class|InteractInterface|Interact(Message) _childactor)
                  (Variables|Default|SetItemAlive false)
                  (goto _label Reset))
                (else
                  (Audio|PlaySoundatLocation "/Game/Sound/Schublade/ClosingDrawer_01.ClosingDrawer_01" (Transformation|GetWorldLocation (Variables|Default|GetSchublade)) "0, 0, 0" 1.0 1.0 0.0 0 0 0)
                  ;[1 1 1] Close Schublade
                  (bind _open_close_2 (Timeline|Timeline_1 ReverseFromEnd)
                    (:Update
                      (Transformation|SetRelativeLocation (Variables|Default|GetSchublade) (Math|Vector|MakeVector (Variables|Default|GetDefault%20X) (Math|Float|Lerp (+ (Variables|Default|GetClose%20Location) 1.0) (Variables|Default|GetOpen%20Location) _open_close_2) (Variables|Default|GetDefault%20Z)) false false)
                      (goto _label_2))
                    (:Finished
                      (Variables|Default|SetIs%20Wardrobe%20Closed true))))))))))))

(event Custom|Destroy_Items
  (bind _collectable (Variables|Default|Getcollectable))
  (bind _childactor (Variables|/Script/Engine.ChildActorComponent|GetChildActor _collectable))
  (if (Utilities|DoesObjectImplementInterface _childactor "/Game/Game/InteractInterFace.InteractInterface_C")
    (Class|InteractInterface|Interact(Message) _childactor)
    (Variables|Default|SetItemAlive false)
    (Utilities|FlowControl|DoOnce false) ; enters at Reset
  ))

(event Custom|SetGameItem
  (params (Target :type Child%20Actor%20Component%20Object%20Reference))
  (bind _new_scale (Variables|Default|GetNew%20Scale))
  (ChildActorComponent|SetChildActorClass Target "/Game/Game/Actors/GameItem.GameItem_C")
  (bind _asgame_item (Utilities|Casting|CastToGameItem (Variables|/Script/Engine.ChildActorComponent|GetChildActor Target)))
  (Variables|/Game/Game/Actors/GameItem.GameItem_C|SetType_E _asgame_item (Variables|Default|GetType_E))
  (Variables|/Game/Game/Actors/GameItem.GameItem_C|SetFood_E _asgame_item (Variables|Default|GetFood_E))
  (Variables|/Game/Game/Actors/GameItem.GameItem_C|SetItem_E _asgame_item (Variables|Default|GetItem_E))
  (Variables|/Game/Game/Actors/GameItem.GameItem_C|SetRecipe_E _asgame_item (Variables|Default|GetRecipe_E))
  (Default|ChangeType _asgame_item)
  (Transformation|SetRelativeScale3D (Variables|/Game/Game/Actors/GameItem.GameItem_C|GetCube _asgame_item) (Math|Vector|MakeVector _new_scale _new_scale _new_scale)))

(event EventBeginPlay
  (bind _collectable (Variables|Default|GetCollectable))
  (bind _schublade (Variables|Default|GetSchublade))
  (bind _relativelocation (Variables|/Script/Engine.SceneComponent|GetRelativeLocation _schublade))
  (bind _relativelocation_2 (Variables|/Script/Engine.SceneComponent|GetRelativeLocation _collectable))
  (bind _relativerotation (Variables|/Script/Engine.SceneComponent|GetRelativeRotation _collectable))
  ;[1 1 1] Set default X & Z Location
  (Variables|Default|SetDefault%20Z (.z _relativelocation))
  (Variables|Default|SetDefault%20X (.x _relativelocation))
  (Variables|Default|SetClose%20Location (.y _relativelocation))
  ;[1 1 1] Randomized Location/Rotation at Spawn
  (Variables|Default|SetItemAlive true)
  (Transformation|SetRelativeLocationAndRotation (Variables|Default|GetCollectable) (Math|Vector|MakeVector (Math|Random|RandomFloatinRange 1e+01 1e+01) (.y _relativelocation_2) (.z _relativelocation_2)) (Math|Rotator|MakeRotator (.roll _relativerotation) (.pitch _relativerotation) (Math|Random|RandomFloatinRange -25.0 25.0)) false false))

(event Collision|EventActorBeginOverlap
  (params (OtherActor :type Actor%20Object%20Reference)))

(event EventTick
  (params (DeltaSeconds :type Float%20%28single-precision%29)))

(fn ConstructionScript)