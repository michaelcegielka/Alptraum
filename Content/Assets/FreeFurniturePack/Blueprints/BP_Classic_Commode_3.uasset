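; Classic commode furniture actor with a drawer that the first-person player can slide open and closed with the Interact input.
; A Box overlap with Roodie_FirstPerson_BP enables input and opens a gate; despite its name, IsLookingAtComm only tracks this overlap.
; After a short delay, Interact runs one of two timelines that lerp the drawer's Y between closed and open positions, toggling IsWardrobeClosed on finish.
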(event OnComponentBeginOverlap(Box)
  (params (OverlappedComponent :type Primitive%20Component%20Object%20Reference) (OtherActor :type Actor%20Object%20Reference) (OtherComp :type Primitive%20Component%20Object%20Reference) (OtherBodyIndex :type Integer) (bFromSweep :type Boolean) (SweepResult :type Hit%20Result%20Structure%20%28by%20ref%29))
  (Utilities|Casting|CastToRoodie_FirstPerson_BP OtherActor)
  (Input|EnableInput (Game|GetPlayerController 0))
  (Variables|Default|SetIsLookingAtComm true)
  (Utilities|FlowControl|Gate true) ; enters at Open
)

(event OnComponentEndOverlap(Box)
  (params (OverlappedComponent :type Primitive%20Component%20Object%20Reference) (OtherActor :type Actor%20Object%20Reference) (OtherComp :type Primitive%20Component%20Object%20Reference) (OtherBodyIndex :type Integer))
  (Utilities|Casting|CastToRoodie_FirstPerson_BP OtherActor)
  (Input|DisableInput (Game|GetPlayerController 0))
  (Variables|Default|SetIsLookingAtComm false)
  (Utilities|FlowControl|Gate true) ; enters at Close
)

(event EventBeginPlay
  (bind _sm_classic_commode_drawer_1_2 (Variables|Default|GetSM_Classic_Commode_Drawer_1_2))
  (bind _relativelocation (Variables|/Script/Engine.SceneComponent|GetRelativeLocation _sm_classic_commode_drawer_1_2))
  ;[1 1 1] Set default X & Z Location
  (Variables|Default|SetLocZ (.z _relativelocation))
  (Variables|Default|SetLocX (.x _relativelocation)))

(event Collision|EventActorBeginOverlap
  (params (OtherActor :type Actor%20Object%20Reference)))

(event EventTick
  (params (DeltaSeconds :type Float%20%28single-precision%29)))

(event Input|ActionEvents|InputActionInteract
  (params (Key :type Key%20Structure :default "None"))
  (:Pressed
    (Utilities|FlowControl|Delay 0.2)
    (if (Variables|Default|GetIsLookingAtComm)
      (Utilities|FlowControl|Gate true
        (:Exit
          (if (Variables|Default|GetIsWardrobeClosed)
            ;[1 1 1] Open Schublade
            (bind _open_close (Timeline|Timeline_0 PlayFromStart)
              (:Update
                (Transformation|SetRelativeLocation (Variables|Default|GetSM_Classic_Commode_Drawer_1_2) (Math|Vector|MakeVector (Variables|Default|GetLocX) (Math|Float|Lerp (Variables|Default|GetCloseLoc) (Variables|Default|GetOpenLoc) _open_close) (Variables|Default|GetLocZ)) false false))
              (:Finished
                (Variables|Default|SetIsWardrobeClosed false)))
            (else
              ;[1 1 1] Close Schublade
              (bind _open_close_2 (Timeline|Timeline_1 ReverseFromEnd)
                (:Update
                  (Transformation|SetRelativeLocation (Variables|Default|GetSM_Classic_Commode_Drawer_1_2) (Math|Vector|MakeVector (Variables|Default|GetLocX) (Math|Float|Lerp (+ (Variables|Default|GetCloseLoc) 1.0) (Variables|Default|GetOpenLoc) _open_close_2) (Variables|Default|GetLocZ)) false false))
                (:Finished
                  (Variables|Default|SetIsWardrobeClosed true))))))))))

(fn ConstructionScript)