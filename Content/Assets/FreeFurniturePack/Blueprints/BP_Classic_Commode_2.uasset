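; Classic commode prop with a drawer the player opens and closes with Interact, holding an optional GameItem.
; The construction script configures the child item's name, type and scale; BeginPlay randomizes its placement or destroys it if unnamed.
; Box overlap with the player enables input and opens a gate; timelines lerp the drawer with sound, debounced by DoOnce.
; Interacting with an open drawer near an item calls the player's ItemRemove instead of closing.
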(event OnComponentBeginOverlap(Box)
  (params (OverlappedComponent :type Primitive%20Component%20Object%20Reference) (OtherActor :type Actor%20Object%20Reference) (OtherComp :type Primitive%20Component%20Object%20Reference) (OtherBodyIndex :type Integer) (bFromSweep :type Boolean) (SweepResult :type Hit%20Result%20Structure%20%28by%20ref%29))
  (Utilities|Casting|CastToRoodie_FirstPerson_BP OtherActor)
  (Input|EnableInput (Game|GetPlayerController 0))
  (Variables|Default|SetIsLookingAtComm true)
  (Utilities|FlowControl|Gate true) ; enters at Open
)

(event OnComponentEndOverlap(Box)
  (params (OverlappedComponent :type Primitive%20Component%20Object%20Reference) (OtherActor :type Actor%20Object%20Reference) (OtherComp :type Primitive%20Component%20Object%20Reference) (OtherBodyIndex :type Integer))
  (Utilities|Casting|CastToRoodie_FirstPerson_BP OtherActor)
  (Input|DisableInput (Game|GetPlayerController 0))
  (Variables|Default|SetIsLookingAtComm false)
  (Utilities|FlowControl|Gate true) ; enters at Close
)

(event EventBeginPlay
  (bind _sm_classic_commode_drawer_1_2 (Variables|Default|GetSM_Classic_Commode_Drawer_1_2))
  (bind _item3 (Variables|Default|Getitem3))
  (bind _relativelocation (Variables|/Script/Engine.SceneComponent|GetRelativeLocation _sm_classic_commode_drawer_1_2))
  (bind _relativelocation_2 (Variables|/Script/Engine.SceneComponent|GetRelativeLocation _item3))
  (bind _relativerotation (Variables|/Script/Engine.SceneComponent|GetRelativeRotation _item3))
  ;[1 1 1] Set default X & Z Location
  (Variables|Default|SetLocZ (.z _relativelocation))
  (Variables|Default|SetLocX (.x _relativelocation))
  ;[1 1 1] Check if a GameItem should exist, else destroy
  (if (Utilities|Name|Equal(Name) (Variables|Default|GetName) "None")
    (Development|PrintString "kein gameItem gesetzt")
    (Actor|DestroyActor (Variables|/Script/Engine.ChildActorComponent|GetChildActor (Variables|Default|Getitem3)))
    (else
      ;[1 1 1] Randomized Location/Rotation at Spawn
      (Transformation|SetRelativeLocationAndRotation (Variables|Default|Getitem3) (Math|Vector|MakeVector (Math|Random|RandomFloatinRange -2e+01 2e+01) (.y _relativelocation_2) (.z _relativelocation_2)) (Math|Rotator|MakeRotator (.roll _relativerotation) (.pitch _relativerotation) (Math|Random|RandomFloatinRange -25.0 25.0)) false false))))

(event Collision|EventActorBeginOverlap
  (params (OtherActor :type Actor%20Object%20Reference)))

(event EventTick
  (params (DeltaSeconds :type Float%20%28single-precision%29)))

(event Input|ActionEvents|InputActionInteract
  (params (Key :type Key%20Structure :default "None"))
  (:Pressed
    (Utilities|FlowControl|Delay 0.2)
    (if (Variables|Default|GetIsLookingAtComm)
      (Utilities|FlowControl|Gate true
        (:Exit
          (Utilities|FlowControl|DoOnce false :!label _label
            (:Completed
              (if (Variables|Default|GetIsWardrobeClosed)
                (Audio|PlaySoundatLocation "/Game/Sound/Schublade/OpeningDrawer01_Cue.OpeningDrawer01_Cue" (Transformation|GetWorldLocation (Variables|Default|GetStaticMesh)) "0, 0, 0" 1.0 1.0 0.0 0 0 0)
                ;[1 1 1] Open Schublade
                (bind _open_close (Timeline|Timeline_0 PlayFromStart)
                  (:Update
                    (Transformation|SetRelativeLocation (Variables|Default|GetSM_Classic_Commode_Drawer_1_2) (Math|Vector|MakeVector (Variables|Default|GetLocX) (Math|Float|Lerp (Variables|Default|GetCloseLoc) (Variables|Default|GetOpenLoc) _open_close) (Variables|Default|GetLocZ)) false false)
                    (Utilities|FlowControl|Delay 2.0 :!label _label_2)
                    (goto _label Reset))
                  (:Finished
                    (Variables|Default|SetIsWardrobeClosed false)))
                (else
                  (bind _asroodie_first_person_bp (Utilities|Casting|CastToRoodie_FirstPerson_BP (Game|GetPlayerCharacter 0)))
                  (if (Variables|/Game/Game/Roodie_BP/Blueprints/Roodie_FirstPerson_BP.Roodie_FirstPerson_BP_C|GetnearItem _asroodie_first_person_bp)
                    (Default|ItemRemove _asroodie_first_person_bp)
                    (Development|PrintString "pick up item first")
                    (goto _label Reset)
                    (else
                      (Audio|PlaySoundatLocation "/Game/Sound/Schublade/ClosingDrawer_01.ClosingDrawer_01" (Transformation|GetWorldLocation (Variables|Default|GetStaticMesh)) "0, 0, 0" 1.0 1.0 0.0 0 0 0)
                      ;[1 1 1] Close Schublade
                      (bind _open_close_2 (Timeline|Timeline_1 ReverseFromEnd)
                        (:Update
                          (Transformation|SetRelativeLocation (Variables|Default|GetSM_Classic_Commode_Drawer_1_2) (Math|Vector|MakeVector (Variables|Default|GetLocX) (Math|Float|Lerp (+ (Variables|Default|GetCloseLoc) 1.0) (Variables|Default|GetOpenLoc) _open_close_2) (Variables|Default|GetLocZ)) false false)
                          (goto _label_2))
                        (:Finished
                          (Variables|Default|SetIsWardrobeClosed true))))))))))))))

(fn ConstructionScript
  (bind _item3 (Variables|Default|Getitem3))
  (bind _new_scale (Variables|Default|GetNew%20Scale))
  (ChildActorComponent|SetChildActorClass _item3 "/Game/Game/Actors/GameItem.GameItem_C")
  (bind _asgame_item (Utilities|Casting|CastToGameItem (Variables|/Script/Engine.ChildActorComponent|GetChildActor _item3)))
  (Variables|/Game/Game/Actors/GameItem.GameItem_C|SetName _asgame_item (Variables|Default|GetName))
  (Default|ChangeType _asgame_item)
  (Transformation|SetRelativeScale3D (Variables|/Game/Game/Actors/GameItem.GameItem_C|GetCube _asgame_item) (Math|Vector|MakeVector _new_scale _new_scale _new_scale)))