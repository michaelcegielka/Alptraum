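; Bed drawer furniture actor that the player opens and closes with the Interact input.
; On BeginPlay it assigns its collectable and openable drawer part to the Collectable and Schublade (drawer) variables, then runs the parent BeginPlay.
; Pressing Interact passes that drawer part and a fixed open offset to OpenClose, whose logic lives outside this graph.
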(event EventBeginPlay
  (Variables|Default|SetCollectable (Variables|Default|GetCollectable1))
  (Variables|Default|SetSchublade (Variables|Default|GetSM_Bed_Drawer_Openable_Part_2))
  (|CallParentFunction))

(event Collision|EventActorBeginOverlap
  (params (OtherActor :type Actor%20Object%20Reference))
  (|CallParentFunction OtherActor) ; This node is disabled and will not be called.\nDrag off pins to build functionality.
)

(event EventTick
  (params (DeltaSeconds :type Float%20%28single-precision%29))
  (|CallParentFunction DeltaSeconds) ; This node is disabled and will not be called.\nDrag off pins to build functionality.
)

(event Input|ActionEvents|InputActionInteract
  (params (Key :type Key%20Structure :default "None"))
  (:Pressed
    (CallFunction|Open/Close 25.0 (Variables|Default|GetSM_Bed_Drawer_Openable_Part_2))))

(fn ConstructionScript
  (|CallParentFunction))