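; Female character Blueprint from a DazToUnreal folder, assembled from modular hair, brow and clothing meshes with a selectable hair color.
; The Construction Script uses HairColor to select Heidi ponytail materials for each Hair slot except slot 1; Violet uses a Front1 material in the Back slot.
; SetMasterPoseFullBody then makes Mesh the master pose component for every part, so all follow its animation.
; The event graph has no active logic.
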(event EventBeginPlay)

(event Collision|EventActorBeginOverlap
  (params (OtherActor :type Actor%20Object%20Reference)))

(event EventTick
  (params (DeltaSeconds :type Float%20%28single-precision%29)))

(fn ConstructionScript
  (bind _hair (Variables|Default|GetHair))
  (bind _haircolor (Variables|Default|GetHairColor))
  (Rendering|Material|SetMaterial _hair 0 (Utilities|Select :Index _haircolor :NewEnumerator0 "/Game/DazToUnreal/Heidi/Heidi_Ponytail_Blond/Materials/Heidi_Ponytail_Blond/Heidi_Ponytail_Blond_Cap.Heidi_Ponytail_Blond_Cap" :NewEnumerator1 "/Game/DazToUnreal/Heidi/Heidi_Ponytail_Blue/Materials/Heidi_Ponytail_Blue/Heidi_Ponytail_Blue_Cap.Heidi_Ponytail_Blue_Cap" :NewEnumerator2 "/Game/DazToUnreal/Heidi/Heidi_Ponytail_Brown/Materials/Leony_Ponytail_Genesis_8_Female/Heidi_Ponytail_Cap.Heidi_Ponytail_Cap" :NewEnumerator3 "/Game/DazToUnreal/Heidi/Heidi_Ponytail_Green/Materials/Heidi_Ponytail_Green/Heidi_Ponytail_Green_Cap.Heidi_Ponytail_Green_Cap" :NewEnumerator4 "/Game/DazToUnreal/Heidi/Heidi_Ponytail_Orange/Materials/Heidi_Ponytail_Orange/Heidi_Ponytail_Orange_Cap.Heidi_Ponytail_Orange_Cap" :NewEnumerator5 "/Game/DazToUnreal/Heidi/Heidi_Ponytail_Pink/Materials/Heidi_Ponytail_Pink/Heidi_Ponytail_Pink_Cap.Heidi_Ponytail_Pink_Cap" :NewEnumerator6 "/Game/DazToUnreal/Heidi/Heidi_Ponytail_Red/Materials/Heidi_Ponytail_Red/Heidi_Ponytail_Red_Cap.Heidi_Ponytail_Red_Cap" :NewEnumerator7 "/Game/DazToUnreal/Heidi/Heidi_Ponytail_Violet/Materials/Heidi_Ponytail_Violet/Heidi_Ponytail_Violet_Cap.Heidi_Ponytail_Violet_Cap"))
  (Rendering|Material|SetMaterial _hair 2 (Utilities|Select :Index _haircolor :NewEnumerator0 "/Game/DazToUnreal/Heidi/Heidi_Ponytail_Blond/Materials/Heidi_Ponytail_Blond/Heidi_Ponytail_Blond_Side2.Heidi_Ponytail_Blond_Side2" :NewEnumerator1 "/Game/DazToUnreal/Heidi/Heidi_Ponytail_Blue/Materials/Heidi_Ponytail_Blue/Heidi_Ponytail_Blue_Side2.Heidi_Ponytail_Blue_Side2" :NewEnumerator2 "/Game/DazToUnreal/Heidi/Heidi_Ponytail_Brown/Materials/Leony_Ponytail_Genesis_8_Female/Heidi_Ponytail_Side2.Heidi_Ponytail_Side2" :NewEnumerator3 "/Game/DazToUnreal/Heidi/Heidi_Ponytail_Green/Materials/Heidi_Ponytail_Green/Heidi_Ponytail_Green_Side2.Heidi_Ponytail_Green_Side2" :NewEnumerator4 "/Game/DazToUnreal/Heidi/Heidi_Ponytail_Orange/Materials/Heidi_Ponytail_Orange/Heidi_Ponytail_Orange_Side2.Heidi_Ponytail_Orange_Side2" :NewEnumerator5 "/Game/DazToUnreal/Heidi/Heidi_Ponytail_Pink/Materials/Heidi_Ponytail_Pink/Heidi_Ponytail_Pink_Side2.Heidi_Ponytail_Pink_Side2" :NewEnumerator6 "/Game/DazToUnreal/Heidi/Heidi_Ponytail_Red/Materials/Heidi_Ponytail_Red/Heidi_Ponytail_Red_Side2.Heidi_Ponytail_Red_Side2" :NewEnumerator7 "/Game/DazToUnreal/Heidi/Heidi_Ponytail_Violet/Materials/Heidi_Ponytail_Violet/Heidi_Ponytail_Violet_Side2.Heidi_Ponytail_Violet_Side2"))
  (Rendering|Material|SetMaterial _hair 3 (Utilities|Select :Index _haircolor :NewEnumerator0 "/Game/DazToUnreal/Heidi/Heidi_Ponytail_Blond/Materials/Heidi_Ponytail_Blond/Heidi_Ponytail_Blond_Side1.Heidi_Ponytail_Blond_Side1" :NewEnumerator1 "/Game/DazToUnreal/Heidi/Heidi_Ponytail_Blue/Materials/Heidi_Ponytail_Blue/Heidi_Ponytail_Blue_Side1.Heidi_Ponytail_Blue_Side1" :NewEnumerator2 "/Game/DazToUnreal/Heidi/Heidi_Ponytail_Brown/Materials/Leony_Ponytail_Genesis_8_Female/Heidi_Ponytail_Side1.Heidi_Ponytail_Side1" :NewEnumerator3 "/Game/DazToUnreal/Heidi/Heidi_Ponytail_Green/Materials/Heidi_Ponytail_Green/Heidi_Ponytail_Green_Side1.Heidi_Ponytail_Green_Side1" :NewEnumerator4 "/Game/DazToUnreal/Heidi/Heidi_Ponytail_Orange/Materials/Heidi_Ponytail_Orange/Heidi_Ponytail_Orange_Side1.Heidi_Ponytail_Orange_Side1" :NewEnumerator5 "/Game/DazToUnreal/Heidi/Heidi_Ponytail_Pink/Materials/Heidi_Ponytail_Pink/Heidi_Ponytail_Pink_Side1.Heidi_Ponytail_Pink_Side1" :NewEnumerator6 "/Game/DazToUnreal/Heidi/Heidi_Ponytail_Red/Materials/Heidi_Ponytail_Red/Heidi_Ponytail_Red_Side1.Heidi_Ponytail_Red_Side1" :NewEnumerator7 "/Game/DazToUnreal/Heidi/Heidi_Ponytail_Violet/Materials/Heidi_Ponytail_Violet/Heidi_Ponytail_Violet_Side1.Heidi_Ponytail_Violet_Side1"))
  (Rendering|Material|SetMaterial _hair 4 (Utilities|Select :Index _haircolor :NewEnumerator0 "/Game/DazToUnreal/Heidi/Heidi_Ponytail_Blond/Materials/Heidi_Ponytail_Blond/Heidi_Ponytail_Blond_Bangs2.Heidi_Ponytail_Blond_Bangs2" :NewEnumerator1 "/Game/DazToUnreal/Heidi/Heidi_Ponytail_Blue/Materials/Heidi_Ponytail_Blue/Heidi_Ponytail_Blue_Bangs2.Heidi_Ponytail_Blue_Bangs2" :NewEnumerator2 "/Game/DazToUnreal/Heidi/Heidi_Ponytail_Brown/Materials/Leony_Ponytail_Genesis_8_Female/Heidi_Ponytail_Bangs2.Heidi_Ponytail_Bangs2" :NewEnumerator3 "/Game/DazToUnreal/Heidi/Heidi_Ponytail_Green/Materials/Heidi_Ponytail_Green/Heidi_Ponytail_Green_Bangs2.Heidi_Ponytail_Green_Bangs2" :NewEnumerator4 "/Game/DazToUnreal/Heidi/Heidi_Ponytail_Orange/Materials/Heidi_Ponytail_Orange/Heidi_Ponytail_Orange_Bangs2.Heidi_Ponytail_Orange_Bangs2" :NewEnumerator5 "/Game/DazToUnreal/Heidi/Heidi_Ponytail_Pink/Materials/Heidi_Ponytail_Pink/Heidi_Ponytail_Pink_Bangs2.Heidi_Ponytail_Pink_Bangs2" :NewEnumerator6 "/Game/DazToUnreal/Heidi/Heidi_Ponytail_Red/Materials/Heidi_Ponytail_Red/Heidi_Ponytail_Red_Bangs2.Heidi_Ponytail_Red_Bangs2" :NewEnumerator7 "/Game/DazToUnreal/Heidi/Heidi_Ponytail_Violet/Materials/Heidi_Ponytail_Violet/Heidi_Ponytail_Violet_Bangs2.Heidi_Ponytail_Violet_Bangs2"))
  (Rendering|Material|SetMaterial _hair 5 (Utilities|Select :Index _haircolor :NewEnumerator0 "/Game/DazToUnreal/Heidi/Heidi_Ponytail_Blond/Materials/Heidi_Ponytail_Blond/Heidi_Ponytail_Blond_Bangs1.Heidi_Ponytail_Blond_Bangs1" :NewEnumerator1 "/Game/DazToUnreal/Heidi/Heidi_Ponytail_Blue/Materials/Heidi_Ponytail_Blue/Heidi_Ponytail_Blue_Bangs1.Heidi_Ponytail_Blue_Bangs1" :NewEnumerator2 "/Game/DazToUnreal/Heidi/Heidi_Ponytail_Brown/Materials/Leony_Ponytail_Genesis_8_Female/Heidi_Ponytail_Bangs1.Heidi_Ponytail_Bangs1" :NewEnumerator3 "/Game/DazToUnreal/Heidi/Heidi_Ponytail_Green/Materials/Heidi_Ponytail_Green/Heidi_Ponytail_Green_Bangs1.Heidi_Ponytail_Green_Bangs1" :NewEnumerator4 "/Game/DazToUnreal/Heidi/Heidi_Ponytail_Orange/Materials/Heidi_Ponytail_Orange/Heidi_Ponytail_Orange_Bangs1.Heidi_Ponytail_Orange_Bangs1" :NewEnumerator5 "/Game/DazToUnreal/Heidi/Heidi_Ponytail_Pink/Materials/Heidi_Ponytail_Pink/Heidi_Ponytail_Pink_Bangs1.Heidi_Ponytail_Pink_Bangs1" :NewEnumerator6 "/Game/DazToUnreal/Heidi/Heidi_Ponytail_Red/Materials/Heidi_Ponytail_Red/Heidi_Ponytail_Red_Bangs1.Heidi_Ponytail_Red_Bangs1" :NewEnumerator7 "/Game/DazToUnreal/Heidi/Heidi_Ponytail_Violet/Materials/Heidi_Ponytail_Violet/Heidi_Ponytail_Violet_Bangs1.Heidi_Ponytail_Violet_Bangs1"))
  (Rendering|Material|SetMaterial _hair 6 (Utilities|Select :Index _haircolor :NewEnumerator0 "/Game/DazToUnreal/Heidi/Heidi_Ponytail_Blond/Materials/Heidi_Ponytail_Blond/Heidi_Ponytail_Blond_BackUnder.Heidi_Ponytail_Blond_BackUnder" :NewEnumerator1 "/Game/DazToUnreal/Heidi/Heidi_Ponytail_Blue/Materials/Heidi_Ponytail_Blue/Heidi_Ponytail_Blue_BackUnder.Heidi_Ponytail_Blue_BackUnder" :NewEnumerator2 "/Game/DazToUnreal/Heidi/Heidi_Ponytail_Brown/Materials/Leony_Ponytail_Genesis_8_Female/Heidi_Ponytail_BackUnder.Heidi_Ponytail_BackUnder" :NewEnumerator3 "/Game/DazToUnreal/Heidi/Heidi_Ponytail_Green/Materials/Heidi_Ponytail_Green/Heidi_Ponytail_Green_BackUnder.Heidi_Ponytail_Green_BackUnder" :NewEnumerator4 "/Game/DazToUnreal/Heidi/Heidi_Ponytail_Orange/Materials/Heidi_Ponytail_Orange/Heidi_Ponytail_Orange_BackUnder.Heidi_Ponytail_Orange_BackUnder" :NewEnumerator5 "/Game/DazToUnreal/Heidi/Heidi_Ponytail_Pink/Materials/Heidi_Ponytail_Pink/Heidi_Ponytail_Pink_BackUnder.Heidi_Ponytail_Pink_BackUnder" :NewEnumerator6 "/Game/DazToUnreal/Heidi/Heidi_Ponytail_Red/Materials/Heidi_Ponytail_Red/Heidi_Ponytail_Red_BackUnder.Heidi_Ponytail_Red_BackUnder" :NewEnumerator7 "/Game/DazToUnreal/Heidi/Heidi_Ponytail_Violet/Materials/Heidi_Ponytail_Violet/Heidi_Ponytail_Violet_BackUnder.Heidi_Ponytail_Violet_BackUnder"))
  (Rendering|Material|SetMaterial _hair 7 (Utilities|Select :Index _haircolor :NewEnumerator0 "/Game/DazToUnreal/Heidi/Heidi_Ponytail_Blond/Materials/Heidi_Ponytail_Blond/Heidi_Ponytail_Blond_Back.Heidi_Ponytail_Blond_Back" :NewEnumerator1 "/Game/DazToUnreal/Heidi/Heidi_Ponytail_Blue/Materials/Heidi_Ponytail_Blue/Heidi_Ponytail_Blue_Back.Heidi_Ponytail_Blue_Back" :NewEnumerator2 "/Game/DazToUnreal/Heidi/Heidi_Ponytail_Brown/Materials/Leony_Ponytail_Genesis_8_Female/Heidi_Ponytail_Back.Heidi_Ponytail_Back" :NewEnumerator3 "/Game/DazToUnreal/Heidi/Heidi_Ponytail_Green/Materials/Heidi_Ponytail_Green/Heidi_Ponytail_Green_Back.Heidi_Ponytail_Green_Back" :NewEnumerator4 "/Game/DazToUnreal/Heidi/Heidi_Ponytail_Orange/Materials/Heidi_Ponytail_Orange/Heidi_Ponytail_Orange_Back.Heidi_Ponytail_Orange_Back" :NewEnumerator5 "/Game/DazToUnreal/Heidi/Heidi_Ponytail_Pink/Materials/Heidi_Ponytail_Pink/Heidi_Ponytail_Pink_Back.Heidi_Ponytail_Pink_Back" :NewEnumerator6 "/Game/DazToUnreal/Heidi/Heidi_Ponytail_Red/Materials/Heidi_Ponytail_Red/Heidi_Ponytail_Red_Back.Heidi_Ponytail_Red_Back" :NewEnumerator7 "/Game/DazToUnreal/Heidi/Heidi_Ponytail_Violet/Materials/Heidi_Ponytail_Violet/Heidi_Ponytail_Violet_Front1.Heidi_Ponytail_Violet_Front1"))
  (Rendering|Material|SetMaterial _hair 8 (Utilities|Select :Index _haircolor :NewEnumerator0 "/Game/DazToUnreal/Heidi/Heidi_Ponytail_Blond/Materials/Heidi_Ponytail_Blond/Heidi_Ponytail_Blond_Front2.Heidi_Ponytail_Blond_Front2" :NewEnumerator1 "/Game/DazToUnreal/Heidi/Heidi_Ponytail_Blue/Materials/Heidi_Ponytail_Blue/Heidi_Ponytail_Blue_Front2.Heidi_Ponytail_Blue_Front2" :NewEnumerator2 "/Game/DazToUnreal/Heidi/Heidi_Ponytail_Brown/Materials/Leony_Ponytail_Genesis_8_Female/Heidi_Ponytail_Front2.Heidi_Ponytail_Front2" :NewEnumerator3 "/Game/DazToUnreal/Heidi/Heidi_Ponytail_Green/Materials/Heidi_Ponytail_Green/Heidi_Ponytail_Green_Front2.Heidi_Ponytail_Green_Front2" :NewEnumerator4 "/Game/DazToUnreal/Heidi/Heidi_Ponytail_Orange/Materials/Heidi_Ponytail_Orange/Heidi_Ponytail_Orange_Front2.Heidi_Ponytail_Orange_Front2" :NewEnumerator5 "/Game/DazToUnreal/Heidi/Heidi_Ponytail_Pink/Materials/Heidi_Ponytail_Pink/Heidi_Ponytail_Pink_Front2.Heidi_Ponytail_Pink_Front2" :NewEnumerator6 "/Game/DazToUnreal/Heidi/Heidi_Ponytail_Red/Materials/Heidi_Ponytail_Red/Heidi_Ponytail_Red_Front2.Heidi_Ponytail_Red_Front2" :NewEnumerator7 "/Game/DazToUnreal/Heidi/Heidi_Ponytail_Violet/Materials/Heidi_Ponytail_Violet/Heidi_Ponytail_Violet_Front2.Heidi_Ponytail_Violet_Front2"))
  (Rendering|Material|SetMaterial _hair 9 (Utilities|Select :Index _haircolor :NewEnumerator0 "/Game/DazToUnreal/Heidi/Heidi_Ponytail_Blond/Materials/Heidi_Ponytail_Blond/Heidi_Ponytail_Blond_Front1.Heidi_Ponytail_Blond_Front1" :NewEnumerator1 "/Game/DazToUnreal/Heidi/Heidi_Ponytail_Blue/Materials/Heidi_Ponytail_Blue/Heidi_Ponytail_Blue_Front1.Heidi_Ponytail_Blue_Front1" :NewEnumerator2 "/Game/DazToUnreal/Heidi/Heidi_Ponytail_Brown/Materials/Leony_Ponytail_Genesis_8_Female/Heidi_Ponytail_Front1.Heidi_Ponytail_Front1" :NewEnumerator3 "/Game/DazToUnreal/Heidi/Heidi_Ponytail_Green/Materials/Heidi_Ponytail_Green/Heidi_Ponytail_Green_Front1.Heidi_Ponytail_Green_Front1" :NewEnumerator4 "/Game/DazToUnreal/Heidi/Heidi_Ponytail_Orange/Materials/Heidi_Ponytail_Orange/Heidi_Ponytail_Orange_Front1.Heidi_Ponytail_Orange_Front1" :NewEnumerator5 "/Game/DazToUnreal/Heidi/Heidi_Ponytail_Pink/Materials/Heidi_Ponytail_Pink/Heidi_Ponytail_Pink_Front1.Heidi_Ponytail_Pink_Front1" :NewEnumerator6 "/Game/DazToUnreal/Heidi/Heidi_Ponytail_Red/Materials/Heidi_Ponytail_Red/Heidi_Ponytail_Red_Front1.Heidi_Ponytail_Red_Front1" :NewEnumerator7 "/Game/DazToUnreal/Heidi/Heidi_Ponytail_Violet/Materials/Heidi_Ponytail_Violet/Heidi_Ponytail_Violet_Front1.Heidi_Ponytail_Violet_Front1"))
  (CallFunction|SetMasterPoseFullBody (Utilities|Array|MakeArray (Variables|Default|GetHair) (Variables|Default|GetBrows) (Variables|Default|GetPanties) (Variables|Default|GetPants) (Variables|Default|GetBra) (Variables|Default|GetTop) (Variables|Default|GetShoes))))

(fn SetMasterPoseFullBody
  (params (NewParam :type Array%20of%20Skinned%20Mesh%20Component%20Object%20References))
  (for _array_element NewParam
    (Class|SkinnedMeshComponent|SetMasterPoseComponent _array_element (Variables|Character|GetMesh) false)))