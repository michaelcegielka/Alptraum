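; AI controller for enemies that runs Enemy_BehaviorTree and passes sightings of the Roodie first-person player to its Blackboard.
; Custom events write the target actor, last location, sight and animation keys.
; On perception updates, a sensed player becomes the target, while a lost one leaves its stimulus location.
; Mannequin_Small pawns update only if CanSee passes, first calling SeePlayerWalk; other pawns update directly.
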(event OnTargetPerceptionUpdated(AIPerception)
  (params (Actor :type Actor%20Object%20Reference) (Stimulus :type AI%20Stimulus%20Structure))
  (bind (_age _expirationage _strength _stimuluslocation _receiverlocation _tag _bsuccessfullysensed) (Utilities|Struct|BreakAIStimulus Stimulus))
  ;[1 1 1] Sight perception
  (bind _asroodie_first_person_bp (Utilities|Casting|CastToRoodie_FirstPerson_BP Actor))
  (bind _asmannequin_small (Utilities|Casting|CastToMannequin_Small (Pawn|GetControlledPawn self))
    (:then
      (bind _cansee (Default|CanSee _asmannequin_small))
      (if _cansee
        (Default|SeePlayerWalk _asmannequin_small)
        (if _bsuccessfullysensed :!label _label
          (CallFunction|SetTargetActor _asroodie_first_person_bp)
          (else
            (CallFunction|SetTargetLocation _stimuluslocation)))
        (CallFunction|SetSeePlayer _bsuccessfullysensed)))
    (:CastFailed
      (goto _label))))

(event Custom|SetTargetActor
  (params (TargetEnemy :type Pawn%20Object%20Reference))
  ;[1 1 1] Set target actor
  (AI|Components|Blackboard|SetValueasObject (Variables|Default|GetBlackboard) (Utilities|Name|MakeLiteralName "TargetActor") TargetEnemy))

(event Custom|SetTargetLocation
  (params (TargetLocation :type Vector))
  ;[1 1 1] Set target location
  (AI|Components|Blackboard|SetValueasVector (Variables|Default|GetBlackboard) (Utilities|Name|MakeLiteralName "TargetLocation") TargetLocation)
  (AI|Components|Blackboard|SetValueasBool (Variables|Default|GetBlackboard) (Utilities|Name|MakeLiteralName "SetLocation") true))

(event Custom|ResetTargetActor
  ;[1 1 1] Reset target actor
  (AI|Components|Blackboard|SetValueasObject (Variables|Default|GetBlackboard) (Utilities|Name|MakeLiteralName "TargetActor") 0))

(event Custom|SetSeePlayer
  (params (BoolValue :type Boolean))
  ;[1 1 1] Set see player
  (AI|Components|Blackboard|SetValueasBool (Variables|Default|GetBlackboard) (Utilities|Name|MakeLiteralName "SeePlayer") BoolValue))

(event Custom|SetDoAnimation
  (params (DoAnimation :type Boolean))
  ;[1 1 1] Set do animation
  (AI|Components|Blackboard|SetValueasBool (Variables|Default|GetBlackboard) (Utilities|Name|MakeLiteralName "DoAnimation") DoAnimation))

(event EventBeginPlay
  ;[1 1 1] set behavior tree
  (AI|RunBehaviorTree "/Game/AI/Enemies/Enemy_BehaviorTree.Enemy_BehaviorTree"))

(fn ConstructionScript)