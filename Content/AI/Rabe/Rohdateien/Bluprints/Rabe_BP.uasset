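; Raven (Rabe) character that wanders the ground and takes flight when the player comes near.
; On BeginPlay it loops AI moves to random nearby reachable points with random pauses until it is flying.
; A Player-tagged sphere overlap sends it straight up with staggered sounds, while IntroFly targets the first FlyGoal actor plus an offset.
; Fly switches the movement mode to Flying, and Tick then steers it toward the stored target.
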(event OnComponentBeginOverlap(Sphere)
  (params (OverlappedComponent :type Primitive%20Component%20Object%20Reference) (OtherActor :type Actor%20Object%20Reference) (OtherComp :type Primitive%20Component%20Object%20Reference) (OtherBodyIndex :type Integer) (bFromSweep :type Boolean) (SweepResult :type Hit%20Result%20Structure%20%28by%20ref%29))
  ;[1 1 1] Fly
  (if (Actor|ActorHasTag OtherActor "Player")
    (CallFunction|RandomFlying "0, 0, 0")
    (Audio|PlaySoundatLocation "/Game/AI/Rabe/Sounds/Rabe_Flügel01_Cue.Rabe_Flügel01_Cue" (Transformation|GetWorldLocation (Variables|Character|GetMesh)) "0, 0, 0" 1.0 1.0 0.0 0 0 0)
    (Utilities|FlowControl|Delay 0.5)
    (Audio|PlaySoundatLocation "/Game/AI/Rabe/Sounds/Rabe_02_Cue.Rabe_02_Cue" (Transformation|GetWorldLocation (Variables|Character|GetMesh)) "0, 0, 0" 1.0 1.0 0.0 0 0 0)
    (Utilities|FlowControl|Delay 1.0)
    (Audio|PlaySoundatLocation "/Game/AI/Rabe/Sounds/Rabe_Background_01.Rabe_Background_01" (Transformation|GetWorldLocation (Variables|Character|GetMesh)) "0, 0, 0" 1.0 1.0 0.0 0 0 0)))

(event Custom|RandomWalk
  ;[1 1 1] Random Walk
  (bind _flying (Class|BPIFlying|IsFlying(Message) self :!label _label))
  (if (not _flying)
    (AI|AIMoveTo self (.RandomLocation (AI|Navigation|GetRandomReachablePointinRadius (Transformation|GetActorLocation) 3e+02 0 0)) 0 5.0 false
      (:then
        _)
      (:OnSuccess
        _)
      (:OnFail
        _))
    (Utilities|FlowControl|Delay (Math|Random|RandomFloatinRange 2.0 1e+01))
    (goto _label)))

(event Custom|IntroFly
  (params (B :type Vector))
  ;[1 1 1] Fly
  (bind _outactors (Actor|GetAllActorsOfClass "/Game/Game/Actors/SequenceStuff/SequenceIntro/FlyGoal.FlyGoal_C"))
  (CallFunction|RandomFlying (+ (.location (Transformation|GetActorTransform (Utilities|Array|Get(acopy) _outactors))) B)))

(event EventBeginPlay
  (CallFunction|RandomWalk))

(event Collision|EventActorBeginOverlap
  (params (OtherActor :type Actor%20Object%20Reference)))

(event EventFly
  (params (TargetLocation :type Vector :default "0, 0, 0"))
  ;[1 1 1] set movement mode
  (Variables|Default|Setfly%20target%20location TargetLocation)
  (Pawn|Components|CharacterMovement|SetMovementMode (Variables|Character|GetCharacterMovement) "MOVE_Flying" 0))

(event EventTick
  (params (DeltaSeconds :type Float%20%28single-precision%29))
  (switch Utilities|FlowControl|Switch|SwitchonEMovementMode (Variables|/Script/Engine.CharacterMovementComponent|GetMovementMode (Variables|Character|GetCharacterMovement))
    (:MOVE_Flying
      (|Flyingmovement))))

(fn ConstructionScript)

(event Custom|Random%20Walk
  (bind _flying (Class|BPIFlying|IsFlying(Message) self :!label _label))
  (if (not _flying)
    (AI|AIMoveTo 0 (.RandomLocation (AI|Navigation|GetRandomReachablePointinRadius (Transformation|GetActorLocation) 3e+02 0 0)) 0 5.0 false
      (:OnSuccess
        _)
      (:OnFail
        _))
    (Utilities|FlowControl|Delay (Math|Random|RandomFloatinRange 2.0 4.0))
    (goto _label)))

(event Custom|Random%20Flying
  (params (Target :type Vector))
  (bind _self self)
  (if (Math|Float|NearlyEqual(Float) (.z Target) 0.0 0.1)
    (Class|BPIFlying|Fly(Message) _self (+ (Transformation|GetActorLocation) "0.000000,0.000000,5000.000000"))
    (else
      (Class|BPIFlying|Fly(Message) _self (Math|Vector|MakeVector (.x Target) (.y Target) (.z Target))))))

(fn IsFlying
  (return (Utilities|Enum|Equal(Enum) (Variables|/Script/Engine.CharacterMovementComponent|GetMovementMode (Variables|Character|GetCharacterMovement)) "MOVE_Flying")))