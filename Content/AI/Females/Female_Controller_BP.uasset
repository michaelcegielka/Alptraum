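; AI controller for female NPCs that runs Female_BehaviorTree on BeginPlay.
; Custom events write to the blackboard, setting or clearing the MissionTarget object and setting the PlayerInRange bool.
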(event Custom|SetMissionTarget
  (params (MissionTarget :type Object%20Object%20Reference))
  ;[1 1 1] Set the new mission
  (AI|Components|Blackboard|SetValueasObject (Variables|Default|GetBlackboard) (Utilities|Name|MakeLiteralName "MissionTarget") MissionTarget))

(event Custom|ResetMissionTarget
  ;[1 1 1] Reset the old mission
  (AI|Components|Blackboard|SetValueasObject (Variables|Default|GetBlackboard) (Utilities|Name|MakeLiteralName "MissionTarget") 0))

(event Custom|SetPlayerInRange
  (params (PlayerInRange :type Boolean))
  ;[1 1 1] Set player in range
  (AI|Components|Blackboard|SetValueasBool (Variables|Default|GetBlackboard) (Utilities|Name|MakeLiteralName "PlayerInRange") PlayerInRange))

(event EventBeginPlay
  ;[1 1 1] Set the behavior tree
  (AI|RunBehaviorTree "/Game/AI/Females/Female_BehaviorTree.Female_BehaviorTree"))

(fn ConstructionScript)