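; Scripted one-shot shadow scare triggered when the first-person Roodie player enters a box volume, gated by a condition flag.
; On BeginPlay it caches outside lights and three doors, found by name.
; The trigger closes and locks both kitchen doors, flickers non-shadow chandeliers, kills outside lights, clears the WindowShadow condition and reveals ShadowRoodie.
; LightOn ends the flicker, restores outside lights and unlocks the second kitchen and shadow doors, leaving the first kitchen door locked.
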(event OnComponentBeginOverlap(Box)
  (params (OverlappedComponent :type Primitive%20Component%20Object%20Reference) (OtherActor :type Actor%20Object%20Reference) (OtherComp :type Primitive%20Component%20Object%20Reference) (OtherBodyIndex :type Integer) (bFromSweep :type Boolean) (SweepResult :type Hit%20Result%20Structure%20%28by%20ref%29))
  (bind _kitchen1 (Variables|Default|GetKitchen1))
  (bind _kitchen2 (Variables|Default|GetKitchen2))
  (Utilities|Casting|CastToRoodie_FirstPerson_BP OtherActor)
  (if (and (Variables|Default|GetFirstTime) (not (Variables|Default|GetCondition)))
    (Utilities|FlowControl|Sequence
      (:then_0
        (if (Variables|/Game/Game/Actors/Doors/Door_BP.Door_BP_C|GetIsClosed _kitchen1)
          _
          (else
            (Default|EventCloseDoor _kitchen1)))
        (Variables|/Game/Game/Actors/Doors/Door_BP.Door_BP_C|SetLoocked _kitchen1 true))
      (:then_1
        (if (Variables|/Game/Game/Actors/Doors/Door_BP.Door_BP_C|GetIsClosed _kitchen2)
          _
          (else
            (Default|EventCloseDoor _kitchen2)))
        (Variables|/Game/Game/Actors/Doors/Door_BP.Door_BP_C|SetLoocked _kitchen2 true))
      (:then_2
        (bind _outactors (Actor|GetAllActorsOfClass "/Game/Assets/EF_FirstFloor/Meshes/Chandelier.Chandelier_C"))
        (for _array_element _outactors
          (if (not (Utilities|Enum|Equal(Enum) (Variables|/Game/Assets/EF_FirstFloor/Meshes/Chandelier.Chandelier_C|GetName _array_element) "shadow"))
            (Default|StartFlickerLight _array_element))))
      (:then_3
        (Variables|/Game/Game/Actors/SequenceStuff/WindowShadow_BP.WindowShadow_BP_C|SetCondition (Variables|Default|GetWindowShadow) false)
        (Variables|Default|SetFirstTime false)
        (for _array_element_2 (Variables|Default|GetLightOutside)
          (Default|TurnLightOff _array_element_2)))
      (:then_4
        (bind _outactors_2 (Actor|GetAllActorsOfClass "/Game/AI/ShadowMan/ShadowRoodie.ShadowRoodie_C"))
        (Rendering|SetActorHiddenInGame (Utilities|Array|Get(acopy) _outactors_2) false)))))

(event Custom|LightOn
  (Variables|/Game/Game/Actors/Doors/Door_BP.Door_BP_C|SetLoocked (Variables|Default|GetKitchen2) false)
  (bind _outactors (Actor|GetAllActorsOfClass "/Game/Assets/EF_FirstFloor/Meshes/Chandelier.Chandelier_C"))
  (for _array_element _outactors
    (if (not (Utilities|Enum|Equal(Enum) (Variables|/Game/Assets/EF_FirstFloor/Meshes/Chandelier.Chandelier_C|GetName _array_element) "shadow"))
      (Default|EndFlicker _array_element)
      (for _array_element_2 (Variables|Default|GetLightOutside)
        (Default|TurnLighton _array_element_2)
        (Variables|/Game/Game/Actors/Doors/Door_BP.Door_BP_C|SetLoocked (Variables|Default|GetDoor) false)))))

(event EventBeginPlay
  (Utilities|FlowControl|Sequence
    (:then_0
      (bind _outactors (Actor|GetAllActorsOfClass "/Game/Game/Actors/Doors/Door_BP.Door_BP_C"))
      (for _array_element _outactors
        (if (Utilities|Enum|Equal(Enum) (Variables|/Game/Game/Actors/Doors/Door_BP.Door_BP_C|GetName _array_element) "kitchen1")
          (Variables|Default|SetKitchen1 _array_element)
          (elif (Utilities|Enum|Equal(Enum) (Variables|/Game/Game/Actors/Doors/Door_BP.Door_BP_C|GetName _array_element) "kitchen2")
            (Variables|Default|SetKitchen2 _array_element)
            (elif (Utilities|Enum|Equal(Enum) (Variables|/Game/Game/Actors/Doors/Door_BP.Door_BP_C|GetName _array_element) "shadow")
              (Variables|Default|SetDoor _array_element))))))
    (:then_1
      (bind _outactors_2 (Actor|GetAllActorsOfClass "/Game/Game/Actors/LightOutside.LightOutside_C"))
      (Variables|Default|SetLightOutside _outactors_2))))

(fn ConstructionScript)