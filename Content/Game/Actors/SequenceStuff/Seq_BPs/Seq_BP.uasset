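; Trigger actor that plays a Level Sequence cutscene when the Roodie first-person player overlaps its box, or when PlaySequence is called.
; Playback runs only while both FirstTime and NeedCondition are false, and sets FirstTime so it cannot repeat.
; During playback the player pawn is hidden with movement disabled.
; A separate EndSequence event restores visibility and walking after a given delay.
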(event OnComponentBeginOverlap(Box)
  (params (OverlappedComponent :type Primitive%20Component%20Object%20Reference) (OtherActor :type Actor%20Object%20Reference) (OtherComp :type Primitive%20Component%20Object%20Reference) (OtherBodyIndex :type Integer) (bFromSweep :type Boolean) (SweepResult :type Hit%20Result%20Structure%20%28by%20ref%29))
  (Utilities|Casting|CastToRoodie_FirstPerson_BP OtherActor)
  (bind _candoit (CallFunction|Condition))
  (if (not _candoit)
    (Utilities|FlowControl|Sequence
      (:then_0
        (Variables|Default|SetFirstTime true)
        (bind _returnvalue (Sequencer|Player|CreateLevelSequencePlayer (Variables|Default|GetLevel%20Sequence)))
        (Sequencer|Player|Play _returnvalue :!class /Script/MovieScene.MovieSceneSequencePlayer))
      (:then_1
        (bind _asroodie_first_person_bp (Utilities|Casting|CastToRoodie_FirstPerson_BP (Game|Player|GetPlayerPawn 0)))
        (Rendering|SetActorHiddenInGame _asroodie_first_person_bp true)
        (Pawn|Components|CharacterMovement|DisableMovement (Variables|/Script/Engine.Character|GetCharacterMovement _asroodie_first_person_bp))))))

(event Custom|PlaySequence
  (bind _candoit (CallFunction|Condition))
  (if (not _candoit)
    (Utilities|FlowControl|Sequence
      (:then_0
        (Variables|Default|SetFirstTime true)
        (bind _returnvalue (Sequencer|Player|CreateLevelSequencePlayer (Variables|Default|GetLevel%20Sequence)))
        (Sequencer|Player|Play _returnvalue :!class /Script/MovieScene.MovieSceneSequencePlayer))
      (:then_1
        (bind _asroodie_first_person_bp (Utilities|Casting|CastToRoodie_FirstPerson_BP (Game|Player|GetPlayerPawn 0)))
        (Rendering|SetActorHiddenInGame _asroodie_first_person_bp true)
        (Pawn|Components|CharacterMovement|DisableMovement (Variables|/Script/Engine.Character|GetCharacterMovement _asroodie_first_person_bp))))))

(event Custom|EndSequence
  (params (Delay :type Float%20%28single-precision%29))
  (Utilities|FlowControl|Delay Delay)
  (bind _asroodie_first_person_bp (Utilities|Casting|CastToRoodie_FirstPerson_BP (Game|Player|GetPlayerPawn 0)))
  (Rendering|SetActorHiddenInGame _asroodie_first_person_bp false)
  (Pawn|Components|CharacterMovement|SetMovementMode (Variables|/Script/Engine.Character|GetCharacterMovement (stale OnComponentBeginOverlap(Box) _asroodie_first_person_bp)) "MOVE_Walking" 0))

(fn ConstructionScript)

(fn Condition
  (return (or (Variables|Default|GetFirstTime) (Variables|Default|GetNeedCondition))))