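; VHS recorder actor that lets the player open a tape-selection widget and change what a linked TV plays.
; BeginPlay loads the player save if it exists; Interact, gated by a DoOnce, debug-prints its video list and opens the player's ChangeVHS widget, or re-arms if empty.
; ChangeVHS assigns the media source to the TV reference.
; ResetVHS collapses the widget, restores game input and resets the gate.
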(event Custom|ChangeVHS
  (params (MediaSource :type Media%20Source%20Object%20Reference))
  ;[1 1 1] Change VHS
  (Variables|/Game/Game/Actors/TV/TVPlayer.TVPlayer_C|SetMediaSource (Variables|Default|GetTV_Reference) MediaSource))

(event Custom|ResetVHS
  (bind _returnvalue (Game|Player|GetPlayerPawn 0))
  (bind _save_ref (Variables|Default|GetSave_Ref))
  (bind _asroodie_first_person_bp (Utilities|Casting|CastToRoodie_FirstPerson_BP _returnvalue))
  (bind _allvideos (Variables|/Game/Game/SaveGamePlayer.SaveGamePlayer_C|GetAllVideos _save_ref))
  (bind _changevhs_ref (Variables|/Game/Game/Roodie_BP/Blueprints/Roodie_FirstPerson_BP.Roodie_FirstPerson_BP_C|GetChangeVHS_Ref _asroodie_first_person_bp))
  ;[1 1 1] Event Interact
  (Widget|SetVisibility _changevhs_ref "Collapsed")
  (Default|InputGame _asroodie_first_person_bp)
  (Utilities|FlowControl|DoOnce false) ; enters at Reset
)

(event EventBeginPlay
  (bind _savegamename (Variables|Default|GetSaveGameName))
  (bind _returnvalue (SaveGame|DoesSaveGameExist _savegamename))
  (if _returnvalue
    (bind _returnvalue_2 (SaveGame|LoadGamefromSlot _savegamename))
    (bind _assave_game_player (Utilities|Casting|CastToSaveGamePlayer _returnvalue_2))
    (Variables|Default|SetSave_Ref _assave_game_player)))

(event Collision|EventActorBeginOverlap
  (params (OtherActor :type Actor%20Object%20Reference)))

(event EventTick
  (params (DeltaSeconds :type Float%20%28single-precision%29)))

(event EventInteract
  (bind _save_ref (Variables|Default|GetSave_Ref))
  (bind _allvideos (Variables|/Game/Game/SaveGamePlayer.SaveGamePlayer_C|GetAllVideos _save_ref))
  ;[1 1 1] Event Interact
  (Utilities|FlowControl|DoOnce false :!label _label
    (:Completed
      (if (== (Utilities|Array|Length _allvideos) 0)
        (Utilities|FlowControl|Delay 0.2)
        (goto _label Reset)
        (else
          (for _array_element _allvideos
            (Development|PrintString (Utilities|String|ToString(Name) _array_element))
            (Default|OpenWidget (Variables|/Game/Game/Roodie_BP/Blueprints/Roodie_FirstPerson_BP.Roodie_FirstPerson_BP_C|GetChangeVHS_Ref (.AsRoodie%20First%20Person%20BP (Utilities|Casting|CastToRoodie_FirstPerson_BP (Game|Player|GetPlayerPawn 0))))))
          (Default|OpenWidget (Variables|/Game/Game/Roodie_BP/Blueprints/Roodie_FirstPerson_BP.Roodie_FirstPerson_BP_C|GetChangeVHS_Ref (.AsRoodie%20First%20Person%20BP (Utilities|Casting|CastToRoodie_FirstPerson_BP (Game|Player|GetPlayerPawn 0))))))))))

(fn ConstructionScript)