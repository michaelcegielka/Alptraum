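; Main menu manager actor that creates and switches between the main menu and its settings pages.
; On BeginPlay it creates the menu, graphics, sound and game settings, achievement and key-in-use widgets, keeps references, and collapses all but the main menu.
; SetNewWidget plays a page-turn sound and shows the chosen page while collapsing the other settings pages, also calling OpenWidget for graphics.
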(event Custom|SetNewWidget
  (params (Visible :type WidgetSettings%20Enum :default "NewEnumerator0"))
  (bind _settings_graphic (Variables|Default|GetSettings%20Graphic))
  (bind _settings_sound (Variables|Default|GetSettings_Sound))
  ;[1 1 1] Set New Widget
  (Audio|PlaySound2D "/Game/Game/UI/Sounds/Menus/SeiteBlättern_Höher.SeiteBlättern_Höher" 1.0 1.0 0.0 0 0)
  (switch Utilities|FlowControl|Switch|SwitchonWidgetSettings Visible
    (:NewEnumerator0
      (Widget|SetVisibility _settings_graphic "Visible")
      (Widget|SetVisibility _settings_sound "Collapsed")
      (Default|OpenWidget _settings_graphic))
    (:NewEnumerator1
      (Widget|SetVisibility _settings_sound "Visible")
      (Widget|SetVisibility _settings_graphic "Collapsed"))
    (:NewEnumerator2
      (Widget|SetVisibility (Variables|Default|GetSettings_Game) "Visible")
      (Widget|SetVisibility _settings_graphic "Collapsed"))
    (:NewEnumerator3
      (Widget|SetVisibility (Variables|Default|GetMainMenu) "Visible")
      (Widget|SetVisibility _settings_graphic "Collapsed"))))

(event EventBeginPlay
  (bind _self self)
  ;[1 1 1] Create Widgets
  (bind _returnvalue (UserInterface|CreateWidget "/Game/Game/UI/MainMenuWidget.MainMenuWidget_C" 0 _self))
  (Variables|Default|SetMainMenu _returnvalue)
  (UserInterface|Viewport|AddtoViewport _returnvalue 0)
  (bind _returnvalue_2 (UserInterface|CreateWidget "/Game/Game/UI/Settings/SettingsGraphicWidget_MainMenu.SettingsGraphicWidget_MainMenu_C" 0 _self))
  (Variables|Default|SetSettings%20Graphic _returnvalue_2)
  (UserInterface|Viewport|AddtoViewport _returnvalue_2 0)
  (bind _returnvalue_3 (UserInterface|CreateWidget "/Game/Game/UI/Settings/SettingsSoundWidget_MainMenu.SettingsSoundWidget_MainMenu_C" 0 _self))
  (Variables|Default|SetSettings_Sound _returnvalue_3)
  (UserInterface|Viewport|AddtoViewport _returnvalue_3 0)
  (bind _returnvalue_4 (UserInterface|CreateWidget "/Game/Game/UI/Settings/SettingsGameWidget_MainMenu.SettingsGameWidget_MainMenu_C" 0 _self))
  (Variables|Default|SetSettings_Game _returnvalue_4)
  (UserInterface|Viewport|AddtoViewport _returnvalue_4 0)
  (bind _returnvalue_5 (UserInterface|CreateWidget "/Game/Game/UI/AchievmentWidget.AchievmentWidget_C" 0 _self))
  (Variables|Default|SetAchievement _returnvalue_5)
  (UserInterface|Viewport|AddtoViewport _returnvalue_5 0)
  (bind _returnvalue_6 (UserInterface|CreateWidget "/Game/Game/UI/Settings/KeyInUseWidget.KeyInUseWidget_C"))
  (Variables|Default|SetKeyInUse_Ref _returnvalue_6)
  (UserInterface|Viewport|AddtoViewport _returnvalue_6 0)
  (Widget|SetVisibility _returnvalue_2 "Collapsed"))

(fn ConstructionScript)