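; Window actor that plays a one-time sound scare when the first-person player overlaps its box trigger.
; The overlap fires once, blocks and stops the level's SoundSystem actor, then plays squeak and laugh sounds at the child actor's location.
; After the squeak's length plus a short delay, it resumes and unblocks the SoundSystem and destroys itself.
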(event OnComponentBeginOverlap(Box)
  (params (OverlappedComponent :type Primitive%20Component%20Object%20Reference) (OtherActor :type Actor%20Object%20Reference) (OtherComp :type Primitive%20Component%20Object%20Reference) (OtherBodyIndex :type Integer) (bFromSweep :type Boolean) (SweepResult :type Hit%20Result%20Structure%20%28by%20ref%29))
  (bind _childactor (Variables|Default|GetChildActor))
  (bind _attenuation_settings (Variables|Default|GetAttenuation%20Settings))
  (bind _quiek (Variables|Default|Getquiek))
  (bind _returnvalue (Transformation|GetWorldLocation _childactor))
  (Utilities|Casting|CastToRoodie_FirstPerson_BP OtherActor)
  (Utilities|FlowControl|DoOnce false
    (:Completed
      (bind _outactors (Actor|GetAllActorsOfClass "/Game/Sound/SoundSystem.SoundSystem_C"))
      (Variables|/Game/Sound/SoundSystem.SoundSystem_C|SetBlocked (Utilities|Array|Get(acopy) _outactors) true)
      (Default|StopSound (Utilities|Array|Get(acopy) _outactors))
      (Audio|PlaySoundatLocation _quiek _returnvalue "0, 0, 0" 1.0 1.0 0.0 _attenuation_settings 0 0)
      (Audio|PlaySoundatLocation (Variables|Default|Getlaugh) _returnvalue "0, 0, 0" 1.0 1.0 0.0 _attenuation_settings 0 0)
      (Utilities|FlowControl|Delay (+ (Variables|/Script/Engine.SoundBase|GetDuration _quiek) 3.0))
      (Default|PlaySound (Utilities|Array|Get(acopy) _outactors))
      (Variables|/Game/Sound/SoundSystem.SoundSystem_C|SetBlocked (Utilities|Array|Get(acopy) _outactors) false)
      (Actor|DestroyActor))))

(event EventBeginPlay)

(event Collision|EventActorBeginOverlap
  (params (OtherActor :type Actor%20Object%20Reference)))

(event EventTick
  (params (DeltaSeconds :type Float%20%28single-precision%29)))

(fn ConstructionScript)