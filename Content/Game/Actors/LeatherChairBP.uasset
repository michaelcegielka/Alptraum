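; Leather chair actor that lets a seated Roodie first-person player control the TV.
; Its box overlap sets or clears the player's Chair reference, and separate events create or remove the TV widget.
; While SitDown is true, Tick polls keys 1–4 to play, pause, resume or close video on the first TVPlayer found, with a button-press montage.
; Held keys retrigger every frame, as the Buttonpress delay logic is unconnected.
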(event OnComponentBeginOverlap(Box)
  (params (OverlappedComponent :type Primitive%20Component%20Object%20Reference) (OtherActor :type Actor%20Object%20Reference) (OtherComp :type Primitive%20Component%20Object%20Reference) (OtherBodyIndex :type Integer) (bFromSweep :type Boolean) (SweepResult :type Hit%20Result%20Structure%20%28by%20ref%29))
  (bind _asroodie_first_person_bp (Utilities|Casting|CastToRoodie_FirstPerson_BP OtherActor))
  (Variables|/Game/Game/Roodie_BP/Blueprints/Roodie_FirstPerson_BP.Roodie_FirstPerson_BP_C|SetChair _asroodie_first_person_bp self))

(event OnComponentEndOverlap(Box)
  (params (OverlappedComponent :type Primitive%20Component%20Object%20Reference) (OtherActor :type Actor%20Object%20Reference) (OtherComp :type Primitive%20Component%20Object%20Reference) (OtherBodyIndex :type Integer))
  (bind _asroodie_first_person_bp (Utilities|Casting|CastToRoodie_FirstPerson_BP OtherActor))
  (Variables|/Game/Game/Roodie_BP/Blueprints/Roodie_FirstPerson_BP.Roodie_FirstPerson_BP_C|SetChair _asroodie_first_person_bp 0))

(event Custom|CreateTVWidget
  (bind _returnvalue (UserInterface|CreateWidget "/Game/Game/UI/TVWidget.TVWidget_C"))
  (UserInterface|Viewport|AddtoViewport _returnvalue 0))

(event Custom|DestroyWidget
  (bind _foundwidgets (Widget|GetAllWidgetsOfClass "/Game/Game/UI/TVWidget.TVWidget_C" false))
  (for _array_element _foundwidgets
    (Widget|RemovefromParent _array_element)))

(event EventTick
  (params (DeltaSeconds :type Float%20%28single-precision%29))
  (bind _returnvalue (Game|GetPlayerController 0))
  (bind _asroodie_first_person_bp (Utilities|Casting|CastToRoodie_FirstPerson_BP (Game|GetPlayerCharacter 0)))
  (if (Variables|/Game/Game/Roodie_BP/Blueprints/Roodie_FirstPerson_BP.Roodie_FirstPerson_BP_C|GetSitDown _asroodie_first_person_bp)
    (bind _outactors (Actor|GetAllActorsOfClass "/Game/Game/Actors/TV/TVPlayer.TVPlayer_C"))
    (if (Game|Player|IsInputKeyDown _returnvalue "One")
      (Default|PlayVideo (Utilities|Array|Get(acopy) _outactors))
      (bind _asroodie_first_person_bp_2 (Utilities|Casting|CastToRoodie_FirstPerson_BP (Game|GetPlayerCharacter 0) :!label _label))
      (Animation|PlayAnimMontage _asroodie_first_person_bp_2 "/Game/Game/Roodie_BP/Animations/ButtonPressAnimMontage.ButtonPressAnimMontage" 2.0 "None")
      (elif (Game|Player|IsInputKeyDown _returnvalue "Two")
        (Default|PauseVideo (Utilities|Array|Get(acopy) _outactors))
        (goto _label)
        (elif (Game|Player|IsInputKeyDown _returnvalue "Three")
          (Default|ResumeVideo (Utilities|Array|Get(acopy) _outactors))
          (goto _label)
          (elif (Game|Player|IsInputKeyDown _returnvalue "Four")
            (Default|CloseVideo (Utilities|Array|Get(acopy) _outactors))
            (goto _label)))))))

(fn ConstructionScript)