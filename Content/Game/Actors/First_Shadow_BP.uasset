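; First_Shadow_BP is a trigger actor that locks selected doors when the Roodie_FirstPerson_BP player enters its Box, apparently for a first shadow event.
; The overlap fires only while Condition is false and FirstTime is true, though neither flag is changed here.
; It searches all Door_BP actors by Name to set Loocked, then searches Chandelier actors by Name without acting on matches.
; The names compared against are empty strings.
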(event OnComponentBeginOverlap(Box)
  (params (OverlappedComponent :type Primitive%20Component%20Object%20Reference) (OtherActor :type Actor%20Object%20Reference) (OtherComp :type Primitive%20Component%20Object%20Reference) (OtherBodyIndex :type Integer) (bFromSweep :type Boolean) (SweepResult :type Hit%20Result%20Structure%20%28by%20ref%29))
  (Utilities|Casting|CastToRoodie_FirstPerson_BP OtherActor)
  (if (and (not (Variables|Default|GetCondition)) (Variables|Default|GetFirstTime))
    (Utilities|FlowControl|Sequence
      (:then_0
        (bind _outactors (Actor|GetAllActorsOfClass "/Game/Game/Actors/Doors/Door_BP.Door_BP_C"))
        (for _array_element _outactors
          (if (or (Utilities|Enum|Equal(Enum) (Variables|/Game/Game/Actors/Doors/Door_BP.Door_BP_C|GetName _array_element) "") (Utilities|Enum|Equal(Enum) (Variables|/Game/Game/Actors/Doors/Door_BP.Door_BP_C|GetName _array_element) ""))
            (Variables|/Game/Game/Actors/Doors/Door_BP.Door_BP_C|SetLoocked _array_element true))))
      (:then_1
        (bind _outactors_2 (Actor|GetAllActorsOfClass "/Game/Game/Actors/Chandelier.Chandelier_C"))
        (for _array_element_2 _outactors_2
          (if (Utilities|Enum|Equal(Enum) (Variables|/Game/Game/Actors/Chandelier.Chandelier_C|Getname _array_element_2) "")
            _))))))

(event EventBeginPlay)

(event Collision|EventActorBeginOverlap
  (params (OtherActor :type Actor%20Object%20Reference)))

(event EventTick
  (params (DeltaSeconds :type Float%20%28single-precision%29)))

(fn ConstructionScript)