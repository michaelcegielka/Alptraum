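; KillPlayer_BP is a trigger actor that sends a lethal Shadow Thing after the player on entering its PlayerInRange box.
; When Roodie_FirstPerson_BP overlaps the box, it spawns TheShadowThing at its own location with Enemy_BehaviorTree and flags it KillPlayer.
; It bypasses normal detection by deactivating AI perception, forcing the player as the seen target on the controller, and overriding walk speed.
; The overlap has no one-shot guard.
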(event OnComponentBeginOverlap(Box_PlayerInRange)
  (params (OverlappedComponent :type Primitive%20Component%20Object%20Reference) (OtherActor :type Actor%20Object%20Reference) (OtherComp :type Primitive%20Component%20Object%20Reference) (OtherBodyIndex :type Integer) (bFromSweep :type Boolean) (SweepResult :type Hit%20Result%20Structure%20%28by%20ref%29))
  (Utilities|Casting|CastToRoodie_FirstPerson_BP OtherActor)
  (bind _returnvalue (AI|SpawnAIFromClass "/Game/AI/Enemies/TheShadowThing/Character/TheShadowThing.TheShadowThing_C" "/Game/AI/Enemies/Enemy_BehaviorTree.Enemy_BehaviorTree" (Transformation|GetActorLocation) "0, 0, 0" true 0))
  (bind _asthe_shadow_thing (Utilities|Casting|CastToTheShadowThing _returnvalue))
  (Variables|/Game/AI/Enemies/TheShadowThing/Character/TheShadowThing.TheShadowThing_C|SetKillPlayer _asthe_shadow_thing true)
  (Components|Activation|Deactivate (Variables|/Game/AI/Enemies/Enemy_Controller_BP.Enemy_Controller_BP_C|GetAIPerception (Variables|/Game/AI/Enemies/TheShadowThing/Character/TheShadowThing.TheShadowThing_C|GetController_Ref _asthe_shadow_thing)))
  (Default|SetTargetActor (Variables|/Game/AI/Enemies/TheShadowThing/Character/TheShadowThing.TheShadowThing_C|GetController_Ref _asthe_shadow_thing) (Game|Player|GetPlayerPawn 0))
  (Default|SetSeePlayer (Variables|/Game/AI/Enemies/TheShadowThing/Character/TheShadowThing.TheShadowThing_C|GetController_Ref _asthe_shadow_thing) true)
  (Variables|/Script/Engine.CharacterMovementComponent|SetMaxWalkSpeed (Variables|/Script/Engine.Character|GetCharacterMovement _asthe_shadow_thing) 8e+02))

(event EventBeginPlay)

(fn ConstructionScript)