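; Interactable hinged door for a horror game that opens and closes, or plays a locked sound when locked.
; Timelines rotate the mesh by DoorPosition, with a slower creaking opening variant and DoOnce gates against repeated triggering; closing always reverses the normal timeline.
; Using an unlocked door flags its number in the GameInstance's per-floor map arrays, and the player's admin mode event unlocks it.
; The construction script sockets both handles and presets open doors.
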(event Custom|OpenAllDoors
  (Variables|Default|SetLoocked false))

(event Custom|OpenCloseDoor
  (bind _door (Variables|Default|GetDoor))
  (bind _returnvalue (Transformation|GetWorldLocation _door))
  (if (not (Variables|Default|GetLoocked))
    (Utilities|FlowControl|DoOnce false :!label _label
      (:Completed
        (CallFunction|SetMapMarker)
        (if (Variables|Default|GetIsClosed)
          (Variables|Default|SetIsClosed false)
          (if (Variables|Default|GetSlow?)
            (Audio|PlaySoundatLocation "/Game/Sound/Tür/Türöffnen01_Cue.Türöffnen01_Cue" _returnvalue "0, 0, 0" 1.0 1.0 0.0 0 0 0)
            (Audio|PlaySoundatLocation "/Game/Sound/Tür/Türquietschen_01_Cue.Türquietschen_01_Cue" _returnvalue "0, 0, 0" 1.0 1.0 0.0 0 0 0)
            (bind _track_opendoor (Timeline|Timeline_1 PlayFromStart)
              (:Update
                (Transformation|SetRelativeRotation (Variables|Default|GetDoor) (Math|Rotator|MakeRotator 0.0 0.0 (* _track_opendoor (Variables|Default|GetDoorPosition))) false false))
              (:Finished
                (Utilities|FlowControl|Delay 1.0 :!label _label_2)
                (goto _label Reset)))
            (else
              (Audio|PlaySoundatLocation "/Game/Sound/Tür/Türöffnen01_Cue.Türöffnen01_Cue" _returnvalue "0, 0, 0" 1.0 1.0 0.0 0 0 0)
              (bind _track_opendoor_2 (Timeline|Timeline_0 PlayFromStart)
                (:Update
                  (Transformation|SetRelativeRotation (Variables|Default|GetDoor) (Math|Rotator|MakeRotator 0.0 0.0 (* _track_opendoor_2 (Variables|Default|GetDoorPosition))) false false))
                (:Finished
                  (goto _label_2)))))
          (else
            (Variables|Default|SetIsClosed true)
            (Timeline|Timeline_0 Reverse)))))
    (else
      (Utilities|FlowControl|DoOnce false :!label _label_3
        (:Completed
          (Audio|PlaySound2D "/Game/Sound/Tür/LockedDoor_01_Cue.LockedDoor_01_Cue" 1.0 1.0 0.0 0 0)
          (Utilities|FlowControl|Delay 1.0)
          (goto _label_3 Reset))))))

(event EventBeginPlay
  (Variables|Default|SetGameinstanceReference (.AsGame%20Instance%20Horror (Utilities|Casting|CastToGameInstanceHorror (Game|GetGameInstance))))
  (EventDispatchers|BindEventtoAdminMode (.AsRoodie%20First%20Person%20BP (Utilities|Casting|CastToRoodie_FirstPerson_BP (Game|Player|GetPlayerPawn 0))) (delegate Custom|OpenAllDoors)))

(event EventInteract
  (bind _door (Variables|Default|GetDoor))
  (bind _returnvalue (Transformation|GetWorldLocation _door))
  (if (not (Variables|Default|GetLoocked))
    (Utilities|FlowControl|DoOnce false :!label _label
      (:Completed
        (CallFunction|SetMapMarker)
        (if (Variables|Default|GetIsClosed)
          (Variables|Default|SetIsClosed false)
          (if (Variables|Default|GetSlow?)
            (Audio|PlaySoundatLocation "/Game/Sound/Tür/Türöffnen01_Cue.Türöffnen01_Cue" _returnvalue "0, 0, 0" 1.0 1.0 0.0 0 0 0)
            (Audio|PlaySoundatLocation "/Game/Sound/Tür/Türquietschen_01_Cue.Türquietschen_01_Cue" _returnvalue "0, 0, 0" 1.0 1.0 0.0 0 0 0)
            (bind _track_opendoor (Timeline|Timeline_1 PlayFromStart)
              (:Update
                (Transformation|SetRelativeRotation (Variables|Default|GetDoor) (Math|Rotator|MakeRotator 0.0 0.0 (* _track_opendoor (Variables|Default|GetDoorPosition))) false false))
              (:Finished
                (Utilities|FlowControl|Delay 1.0 :!label _label_2)
                (goto _label Reset)))
            (else
              (Audio|PlaySoundatLocation "/Game/Sound/Tür/Türöffnen01_Cue.Türöffnen01_Cue" _returnvalue "0, 0, 0" 1.0 1.0 0.0 0 0 0)
              (bind _track_opendoor_2 (Timeline|Timeline_0 PlayFromStart)
                (:Update
                  (Transformation|SetRelativeRotation (Variables|Default|GetDoor) (Math|Rotator|MakeRotator 0.0 0.0 (* _track_opendoor_2 (Variables|Default|GetDoorPosition))) false false))
                (:Finished
                  (goto _label_2)))))
          (else
            (Variables|Default|SetIsClosed true)
            (Timeline|Timeline_0 Reverse)))))
    (else
      (Utilities|FlowControl|DoOnce false :!label _label_3
        (:Completed
          (Audio|PlaySound2D "/Game/Sound/Tür/LockedDoor_01_Cue.LockedDoor_01_Cue" 1.0 1.0 0.0 0 0)
          (Utilities|FlowControl|Delay 1.0)
          (goto _label_3 Reset))))))

(event EventInteractJ
  (Utilities|FlowControl|DoOnce false :!label _label
    (:Completed
      (Audio|PlaySound2D "/Game/Sound/Tür/LockedDoor_01_Cue.LockedDoor_01_Cue" 1.0 1.0 0.0 0 0)
      (Utilities|FlowControl|Delay 1.0)
      (goto _label Reset))))

(fn ConstructionScript
  (bind _door (Variables|Default|GetDoor))
  (Transformation|AttachComponentToComponent (Variables|Default|GetHandleR) _door "HandleRight" "KeepRelative" "KeepRelative" "KeepRelative" true)
  (Transformation|AttachComponentToComponent (Variables|Default|GetHandleL) _door "HandleLeft" "KeepRelative" "KeepRelative" "KeepRelative" true)
  (if (not (Variables|Default|GetIsClosed))
    (Transformation|SetRelativeRotation (Variables|Default|GetDoor) (Math|Rotator|MakeRotator 0.0 0.0 (Variables|Default|GetDoorPosition)) false false)))

(fn SetMapMarker
  (bind _gameinstancereference (Variables|Default|GetGameinstanceReference))
  (bind _number (Variables|Default|GetNumber))
  (switch Utilities|FlowControl|Switch|SwitchonPositionEnum (Variables|Default|GetFloorPosition)
    (:NewEnumerator0
      (Utilities|Array|SetArrayElem (Variables|/Game/Game/GameInstanceHorror.GameInstanceHorror_C|GetChekedDoorsEG _gameinstancereference) _number true true))
    (:NewEnumerator1
      (Utilities|Array|SetArrayElem (Variables|/Game/Game/GameInstanceHorror.GameInstanceHorror_C|GetChekedDoorsDG _gameinstancereference) _number true true))
    (:NewEnumerator5
      (Utilities|Array|SetArrayElem (Variables|/Game/Game/GameInstanceHorror.GameInstanceHorror_C|GetChekedDoorsE0 _gameinstancereference) _number true true))
    (:NewEnumerator2
      (Utilities|Array|SetArrayElem (Variables|/Game/Game/GameInstanceHorror.GameInstanceHorror_C|GetChekedDoorsE1 _gameinstancereference) _number true true))
    (:NewEnumerator3
      (Utilities|Array|SetArrayElem (Variables|/Game/Game/GameInstanceHorror.GameInstanceHorror_C|GetChekedDoorsE2 _gameinstancereference) _number true true))))