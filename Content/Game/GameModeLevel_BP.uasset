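; GameModeLevel_BP is a level game mode that sets up the player's UI and links key actors at BeginPlay.
; It caches the Roodie first-person pawn and the first VHS recorder in the level, then creates the overlay widget and adds it to the viewport.
; The overlay's change-video widget receives the recorder reference, and the pawn is switched to game input and given a reference to the game mode.
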(event Custom|GetAllActors
  (bind _asroodie_first_person_bp (Utilities|Casting|CastToRoodie_FirstPerson_BP (Game|Player|GetPlayerPawn 0)))
  (Variables|Default|SetPlayer_Ref _asroodie_first_person_bp)
  (bind _outactors (Actor|GetAllActorsOfClass "/Game/Game/Actors/TV/VHS_Recorder_BP.VHS_Recorder_BP_C"))
  (Variables|Default|SetVHS_Ref (Utilities|Array|Get(acopy) _outactors)))

(event Custom|CreateAllWidgets
  (CallFunction|GetAllActors)
  (bind _returnvalue (UserInterface|CreateWidget "/Game/Game/UI/Overlay_W.Overlay_W_C" (Game|GetPlayerController 0)))
  (bind _output_get (Variables|Default|SetOverlay_W _returnvalue))
  (UserInterface|Viewport|AddtoViewport _output_get 0)
  (Variables|/Game/Game/UI/ChangeVideoWidget.ChangeVideoWidget_C|SetVHS_Recorder_Reference (Variables|/Game/Game/UI/Overlay_W.Overlay_W_C|GetChangeVideoWidget _returnvalue) (Variables|Default|GetVHS_Ref)))

(event EventBeginPlay
  (CallFunction|CreateAllWidgets)
  (bind _asroodie_first_person_bp (Utilities|Casting|CastToRoodie_FirstPerson_BP (Game|Player|GetPlayerPawn 0)))
  (Default|InputGame _asroodie_first_person_bp)
  (Variables|/Game/Game/Roodie_BP/Blueprints/Roodie_FirstPerson_BP.Roodie_FirstPerson_BP_C|SetGameMode_Ref _asroodie_first_person_bp self))

(fn ConstructionScript)